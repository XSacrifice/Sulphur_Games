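; Exit door actor for the Dark2Floors map that opens once enough collect points are gathered, and also runs a gas hazard on the player.
; CollectPoint counts toward a maximum, then fires OpenDoor once, sliding the door along X with a timeline.
; Gas starts an endless delay loop that damages the player every two seconds and stacks WB_GAS widgets on screen up to a cap of five.
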(event Custom|Open%20Door
  (bind _door_ratation (Timeline|Open%20Door%20Anim Play)
    (:Update
      (Transformation|SetRelativeLocation (Variables|Default|GetDoor) (Math|Vector|MakeVector (Math|Float|Lerp 2.6e+02 -2e+02 _door_ratation) 0.0 0.0) false false))))

(event Custom|CollectPoint
  (Math|Integer|IncrementInt (Variables|Default|GetCollectPointToOpen)
    (:%20%20
      (if (>= (Variables|Default|GetCollectPointToOpen) (Variables|Default|GetMaxCollectPointToOpen))
        (Utilities|FlowControl|DoOnce false
          (:Completed
            (CallFunction|OpenDoor)))))))

(event Custom|Gas
  (bind _asbp_player (Utilities|Casting|CastToBP_Player (Game|GetPlayerCharacter 0)))
  (Utilities|FlowControl|Delay 2.0 :!label _label)
  (Game|Damage|ApplyDamage _asbp_player 5.0 0 0)
  (if (== (Variables|Default|GetUIgas) 5)
    (goto _label)
    (else
      (bind _returnvalue (UserInterface|CreateWidget "/Game/ThirdPerson/UI/WB_GAS.WB_GAS_C"))
      (UserInterface|Viewport|AddtoViewport _returnvalue 0)
      (Math|Integer|IncrementInt (Variables|Default|GetUIgas)
        (:%20%20
          (goto _label))))))

(fn ConstructionScript)