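; Armored zombie enemy character that melees the player, takes damage and drops loot on death.
; A sphere overlap gates attacks from checkplayer; the montage attack applies delayed damage when the hand boxes have flagged the player.
; AnyDamage reduces health, then on death ragdolls the mesh with an impulse away from the damage causer and destroys it after a delay.
; DropLoot spawns scrap plus chance-based pistol ammo; a skill-scrap drop variant is never called here.
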(event OnComponentBeginOverlap(BoxR)
  (params (OverlappedComponent :type Primitive%20Component%20Object%20Reference) (OtherActor :type Actor%20Object%20Reference) (OtherComp :type Primitive%20Component%20Object%20Reference) (OtherBodyIndex :type Integer) (bFromSweep :type Boolean) (SweepResult :type Hit%20Result%20Structure%20%28by%20ref%29))
  ;[1 1 1] Attack Check
  (Utilities|Casting|CastToBP_Player OtherActor
    (:then
      (Variables|Default|Setin%20box? true))
    (:CastFailed
      (Variables|Default|Setin%20box? false))))

(event OnComponentBeginOverlap(BoxL)
  (params (OverlappedComponent :type Primitive%20Component%20Object%20Reference) (OtherActor :type Actor%20Object%20Reference) (OtherComp :type Primitive%20Component%20Object%20Reference) (OtherBodyIndex :type Integer) (bFromSweep :type Boolean) (SweepResult :type Hit%20Result%20Structure%20%28by%20ref%29))
  ;[1 1 1] Attack Check
  (Utilities|Casting|CastToBP_Player OtherActor
    (:then
      (Variables|Default|Setin%20box? true))
    (:CastFailed
      (Variables|Default|Setin%20box? false))))

(event OnComponentBeginOverlap(Sphere)
  (params (OverlappedComponent :type Primitive%20Component%20Object%20Reference) (OtherActor :type Actor%20Object%20Reference) (OtherComp :type Primitive%20Component%20Object%20Reference) (OtherBodyIndex :type Integer) (bFromSweep :type Boolean) (SweepResult :type Hit%20Result%20Structure%20%28by%20ref%29))
  (Utilities|Casting|CastToBP_Player OtherActor)
  (Variables|Default|SetZombie%20Can%20Attack true))

(event OnComponentEndOverlap(Sphere)
  (params (OverlappedComponent :type Primitive%20Component%20Object%20Reference) (OtherActor :type Actor%20Object%20Reference) (OtherComp :type Primitive%20Component%20Object%20Reference) (OtherBodyIndex :type Integer))
  (Utilities|Casting|CastToBP_Player OtherActor)
  (Variables|Default|SetZombie%20Can%20Attack false))

(event Custom|Droploot%20SkillCard
  (bind _returnvalue (Transformation|GetActorLocation))
  ;[1 1 1] Drop (Skill)
  (Variables|Default|SetIsDropped? true)
  (Game|SpawnActorfromClass "/Game/Shop/Scrap/BP_SScrap.BP_SScrap_C" (Math|Conversions|ToTransform(Vector) (- _returnvalue "0.000000,0.000000,100.000000")) "AlwaysSpawn" "MultiplyWithRoot" 0 0)
  (bind _outhit (Collision|LineTraceByChannel _returnvalue (- _returnvalue "0.000000,0.000000,200.000000") "TraceTypeQuery1" false (Utilities|Array|MakeArray (Game|GetPlayerCharacter 0)) "None"))
  (Game|SpawnActorfromClass (Utilities|Select :Index (Math|Random|RandomInteger 5) :Option%200 "/Game/Shop/Scrap/BP_SScrap.BP_SScrap_C" :Option%201 0 :Option%202 0 :Option%203 0 :Option%204 0) (Math|Transform|MakeTransform (.Location (Collision|BreakHitResult _outhit)) (Math|Rotator|MakeRotator 0.0 0.0 (Math|Random|RandomFloatinRange 0.0 3.6e+02))) "AlwaysSpawn" "MultiplyWithRoot" 0 0))

(event Custom|Attack
  ;[1 1 1] Attack
  (if (not (Variables|Default|GetIsDead?))
    (Animation|PlayAnimMontage "/Game/Characters_Added/Zombie/03_Armored/Mesh/Animation/Armored_Attack_Montage.Armored_Attack_Montage" 1.0 "None")
    (Utilities|FlowControl|Sequence
      (:then_0
        (Utilities|FlowControl|Delay 0.2)
        (Audio|PlaySoundatLocation "/Game/Sound/Human/Armored_Hit.Armored_Hit" (Transformation|GetActorLocation) "0, 0, 0" 1.0 1.0 0.0 0 0 0 0)
        (Variables|Default|SetHit? true))
      (:then_1
        (Utilities|FlowControl|Delay 0.8)
        (CallFunction|Hit)))))

(event Custom|Hit
  ;[1 1 1] Attack Check
  (if (not (Variables|Default|GetIsDead?))
    (if (Variables|Default|GetHit?)
      (if (Variables|Default|Getin%20box?)
        (Utilities|FlowControl|Delay 0.1)
        (Game|Damage|ApplyDamage (Variables|Default|GetAs%20BP%20Third%20Person%20Character) 3e+01 0 self)
        (Default|PlayerGotDamage (Variables|Default|GetAs%20BP%20Third%20Person%20Character))))))

(event Custom|DropLoot
  (bind _returnvalue (Transformation|GetActorLocation))
  ;[1 1 1] Drop Loot
  (Variables|Default|SetIsDropped? true)
  (Game|SpawnActorfromClass "/Game/Shop/Scrap/BP_BScrap.BP_BScrap_C" (Math|Conversions|ToTransform(Vector) (- _returnvalue "0.000000,0.000000,100.000000")) "AlwaysSpawn" "MultiplyWithRoot" 0 0)
  (bind _outhit (Collision|LineTraceByChannel _returnvalue (- _returnvalue "0.000000,0.000000,200.000000") "TraceTypeQuery1" false (Utilities|Array|MakeArray (Game|GetPlayerCharacter 0)) "None"))
  (Game|SpawnActorfromClass (Utilities|Select :Index (Math|Random|RandomInteger 8) :Option%200 "/Game/ThirdPerson/Blueprints/Item/BP_PistolAmmoPickuup_3.BP_PistolAmmoPickuup_3_C" :Option%201 0 :Option%202 0 :Option%203 0 :Option%204 0 :Option%205 0 :Option%206 0 :Option%207 0 :Option%208 0) (Math|Transform|MakeTransform (.Location (Collision|BreakHitResult _outhit)) (Math|Rotator|MakeRotator 0.0 0.0 (Math|Random|RandomFloatinRange 0.0 3.6e+02))) "AlwaysSpawn" "MultiplyWithRoot" 0 0))

(event Custom|check%20player
  ;[1 1 1] Attack Check
  (if (Variables|Default|GetZombie%20Can%20Attack)
    (CallFunction|Attack)))

(event EventBeginPlay
  (bind _asbp_player (Utilities|Casting|CastToBP_Player (Game|GetPlayerCharacter 0)))
  (Variables|Default|SetAs%20BP%20Third%20Person%20Character _asbp_player)
  (if (== (Variables|Default|GetCurrentHealth_Armored) 0.0)
    (Actor|DestroyActor)
    (else
      (Variables|Default|SetCurrentHealth_Armored (Variables|Default|GetMaxHealth_Armored)))))

(event Game|Damage|EventAnyDamage
  (params (Damage :type Float%20%28single-precision%29) (DamageType :type Damage%20Type%20Object%20Reference) (InstigatedBy :type Controller%20Object%20Reference) (DamageCauser :type Actor%20Object%20Reference))
  (bind _mesh (Variables|Character|GetMesh))
  ;[1 1 1] Dead
  (Variables|Default|SetDamage%20Causer DamageCauser)
  (Audio|PlaySoundatLocation "/Game/MilitaryWeapDark/Sound/Shotgun/Shotgun_ImpactBody_Cue.Shotgun_ImpactBody_Cue" (Transformation|GetActorLocation) "0, 0, 0" 1.0 1.0 0.0 0 0 0 0)
  (bind _output_get (Variables|Default|SetCurrentHealth_Armored (- (Variables|Default|GetCurrentHealth_Armored) Damage)))
  (if (<= _output_get 0.0)
    (if (Variables|Default|GetIsDead?)
      (Variables|Default|SetIsDropped? true)
      (else
        (Audio|PlaySoundatLocation "/Game/Sound/Human/HugeZDeath.HugeZDeath" (Transformation|GetActorLocation) "0, 0, 0" 1.0 1.0 0.0 0 0 0 0)))
    (for _index (range 0 (Math|Random|RandomInteger 2))
      (if (not (Variables|Default|GetIsDead?))
        (if (not (Variables|Default|GetIsDropped?))
          (CallFunction|DropLoot))))
    (Pawn|Components|CharacterMovement|DisableMovement (Variables|Character|GetCharacterMovement))
    (Variables|Default|SetIsDead? true)
    (Physics|SetSimulatePhysics _mesh true)
    (Physics|AddImpulse _mesh (* (Math|Vector|Normalize (- (Transformation|GetActorLocation) (Transformation|GetActorLocation (Variables|Default|GetDamage%20Causer)))) 300) "None" true)
    (Collision|SetCollisionResponsetoChannel (Variables|Character|GetMesh) "ECC_PhysicsBody" "ECR_Ignore")
    (Collision|SetCollisionResponsetoChannel (Variables|Character|GetMesh) "ECC_Pawn" "ECR_Ignore")
    (Utilities|FlowControl|Delay 8.0)
    (Actor|DestroyActor)
    (elif (not (Variables|Default|GetIsDead?))
      (Audio|PlaySoundatLocation "/Game/Sound/Human/Cue/BIGZGruntCue.BIGZGruntCue" (Transformation|GetActorLocation) "0, 0, 0" 1.0 1.0 0.0 0 0 0 0))))

(fn ConstructionScript)