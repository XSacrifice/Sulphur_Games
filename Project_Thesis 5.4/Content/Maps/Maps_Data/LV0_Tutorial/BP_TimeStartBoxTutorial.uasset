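; Tutorial trigger box that starts the timer when something overlaps it, with no filter on the overlapping actor.
; A DoOnce on the Box overlap waits briefly, then adds WB_TimerTutorial to the viewport, calls its StartGame and sets AlreadyCountDown.
; If that flag is already set when the DoOnce fires, the actor destroys itself instead.
; An unconnected branch that would show WB_LootStart never runs.
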(event OnComponentBeginOverlap(Box)
  (params (OverlappedComponent :type Primitive%20Component%20Object%20Reference) (OtherActor :type Actor%20Object%20Reference) (OtherComp :type Primitive%20Component%20Object%20Reference) (OtherBodyIndex :type Integer) (bFromSweep :type Boolean) (SweepResult :type Hit%20Result%20Structure%20%28by%20ref%29))
  (Utilities|FlowControl|DoOnce false
    (:Completed
      (if (Variables|Default|GetAlreadyCountDown?)
        (Actor|DestroyActor)
        (else
          (Utilities|FlowControl|Sequence
            (:then_0
              (Utilities|FlowControl|Delay 0.1)
              (bind _returnvalue (UserInterface|CreateWidget "/Game/Characters/Player/Blueprint/Widget/WB_TimerTutorial.WB_TimerTutorial_C"))
              (if true
                (UserInterface|Viewport|AddtoViewport _returnvalue 0)
                (Default|StartGame _returnvalue)
                (Variables|Default|SetAlreadyCountDown? true)))))))))

(event EventBeginPlay)

(event Collision|EventActorBeginOverlap
  (params (OtherActor :type Actor%20Object%20Reference)))

(event EventPlayerInteracted
  (params (Player :type BP%20Player%20Object%20Reference)))

(fn ConstructionScript)