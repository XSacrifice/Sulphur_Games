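; BP_ObjectiveSpawner is a one-shot spawner actor that places a BP_Objective_Global in the level.
; StartSpawn sets a timer, and SpawnObjective spawns the objective at the Arrow component's world transform, then destroys the spawner.
; An unconnected branch that would spawn AI from ObjectType up to a MaxObject count never runs.
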(event Custom|SpawnObjective
  (Game|SpawnActorfromClass "/Game/Maps/Maps_Data/GAME_CONTROLLER/BP_Objective_Global.BP_Objective_Global_C" (Transformation|GetWorldTransform (Variables|Default|GetArrow)) "Undefined" "MultiplyWithRoot" 0 0)
  (Actor|DestroyActor))

(event Custom|StartSpawn
  (Utilities|Time|SetTimerbyEvent 0 (Variables|Default|GetTime)))

(fn ConstructionScript)