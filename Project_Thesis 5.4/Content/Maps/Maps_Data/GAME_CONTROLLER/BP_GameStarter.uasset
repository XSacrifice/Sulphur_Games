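; BP_GameStarter is a one-shot trigger actor that starts the game when something overlaps its Box.
; A DoOnce feeds a Sequence that calls CollectPoint on all BP_DEnter_Global actors and shows the WDG_GameStarter and WB_LootStart widgets, calling their start functions.
; Only the game-starter widget waits on a short Delay, so the loot widget appears first and the Box is destroyed immediately.
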(event OnComponentBeginOverlap(Box)
  (params (OverlappedComponent :type Primitive%20Component%20Object%20Reference) (OtherActor :type Actor%20Object%20Reference) (OtherComp :type Primitive%20Component%20Object%20Reference) (OtherBodyIndex :type Integer) (bFromSweep :type Boolean) (SweepResult :type Hit%20Result%20Structure%20%28by%20ref%29))
  (Utilities|FlowControl|DoOnce false
    (:Completed
      (Utilities|FlowControl|Sequence
        (:then_0
          (bind _outactors (Actor|GetAllActorsOfClass "/Game/Maps/Maps_Data/GAME_CONTROLLER/BP_DEnter_Global.BP_DEnter_Global_C"))
          (Default|CollectPoint _outactors))
        (:then_1
          (Utilities|FlowControl|Delay 0.2)
          (bind _returnvalue (UserInterface|CreateWidget "/Game/Maps/Maps_Data/GAME_CONTROLLER/WDG_GameStarter.WDG_GameStarter_C"))
          (UserInterface|Viewport|AddtoViewport _returnvalue 0)
          (Default|StartGame _returnvalue))
        (:then_2
          (bind _returnvalue_2 (UserInterface|CreateWidget "/Game/Characters/Player/Blueprint/Widget/WB_LootStart.WB_LootStart_C"))
          (UserInterface|Viewport|AddtoViewport _returnvalue_2 0)
          (Default|LootStart _returnvalue_2))
        (:then_3
          (Components|DestroyComponent (Variables|Default|GetBox)))))))

(event EventBeginPlay)

(event Collision|EventActorBeginOverlap
  (params (OtherActor :type Actor%20Object%20Reference)))

(event EventTick
  (params (DeltaSeconds :type Float%20%28single-precision%29)))

(fn ConstructionScript)