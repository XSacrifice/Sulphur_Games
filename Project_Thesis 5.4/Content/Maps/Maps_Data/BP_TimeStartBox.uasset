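; BP_TimeStartBox is a map trigger volume that starts the countdown and loot start UI when the player enters it.
; A box overlap by BP_Player passes a DoOnce, then destroys the actor if AlreadyCountDown is already set.
; Otherwise it shows and starts WB_LootStart immediately and WB_MSewerTimer after a short delay, with both branches setting AlreadyCountDown.
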(event OnComponentBeginOverlap(Box)
  (params (OverlappedComponent :type Primitive%20Component%20Object%20Reference) (OtherActor :type Actor%20Object%20Reference) (OtherComp :type Primitive%20Component%20Object%20Reference) (OtherBodyIndex :type Integer) (bFromSweep :type Boolean) (SweepResult :type Hit%20Result%20Structure%20%28by%20ref%29))
  (Utilities|Casting|CastToBP_Player OtherActor)
  (Utilities|FlowControl|DoOnce false
    (:Completed
      (if (Variables|Default|GetAlreadyCountDown?)
        (Actor|DestroyActor)
        (else
          (Utilities|FlowControl|Sequence
            (:then_0
              (Utilities|FlowControl|Delay 0.2)
              (bind _returnvalue (UserInterface|CreateWidget "/Game/Maps/Maps_Data/LV4_Main_Sewer/WB_MSewerTimer.WB_MSewerTimer_C"))
              (if true
                (UserInterface|Viewport|AddtoViewport _returnvalue 0)
                (Default|StartGame _returnvalue)
                (Variables|Default|SetAlreadyCountDown? true)))
            (:then_1
              (bind _returnvalue_2 (UserInterface|CreateWidget "/Game/Characters/Player/Blueprint/Widget/WB_LootStart.WB_LootStart_C"))
              (UserInterface|Viewport|AddtoViewport _returnvalue_2 0)
              (Default|LootStart _returnvalue_2)
              (Variables|Default|SetAlreadyCountDown? true))))))))

(event Collision|EventActorBeginOverlap
  (params (OtherActor :type Actor%20Object%20Reference)))

(fn ConstructionScript)