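; BP_TimeStartBoxH6 is an LV6 trigger box that starts the HS6 timer when the player overlaps it.
; The overlap fires only once, with the player cast after the DoOnce, so any first overlapping actor consumes the trigger.
; For BP_Player, it immediately shows WB_LootStart and calls LootStart, while WB_TimerHS6 appears and runs StartGame after a short delay.
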(event OnComponentBeginOverlap(Box)
  (params (OverlappedComponent :type Primitive%20Component%20Object%20Reference) (OtherActor :type Actor%20Object%20Reference) (OtherComp :type Primitive%20Component%20Object%20Reference) (OtherBodyIndex :type Integer) (bFromSweep :type Boolean) (SweepResult :type Hit%20Result%20Structure%20%28by%20ref%29))
  (Utilities|FlowControl|DoOnce false
    (:Completed
      (Utilities|Casting|CastToBP_Player OtherActor)
      (Utilities|FlowControl|Sequence
        (:then_0
          (Utilities|FlowControl|Delay 0.2)
          (bind _returnvalue (UserInterface|CreateWidget "/Game/Maps/Maps_Data/LV6/WB_TimerHS6.WB_TimerHS6_C"))
          (if true
            (UserInterface|Viewport|AddtoViewport _returnvalue 0)
            (Default|StartGame _returnvalue)))
        (:then_1
          (bind _returnvalue_2 (UserInterface|CreateWidget "/Game/Characters/Player/Blueprint/Widget/WB_LootStart.WB_LootStart_C"))
          (UserInterface|Viewport|AddtoViewport _returnvalue_2 0)
          (Default|LootStart _returnvalue_2))))))

(event EventBeginPlay)

(event Collision|EventActorBeginOverlap
  (params (OtherActor :type Actor%20Object%20Reference)))

(event EventPlayerInteracted
  (params (Player :type BP%20Player%20Object%20Reference)))

(fn ConstructionScript)