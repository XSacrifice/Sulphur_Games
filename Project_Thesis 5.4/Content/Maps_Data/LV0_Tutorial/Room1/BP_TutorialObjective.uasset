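; Tutorial objective button that the player activates once by pressing E to score a point toward the tutorial exit.
; A box overlap with BP_Player enables input and shows a press-E widget; leaving reverses both.
; Pressing E plays a click, swaps the lights, destroys the box and calls CollectPoint on BP_DExitTutorial.
; Hold-to-activate timer logic and an ObjectiveSpawnner4 spawn call remain but are disconnected.
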(event OnComponentBeginOverlap(Box)
  (params (OverlappedComponent :type Primitive%20Component%20Object%20Reference) (OtherActor :type Actor%20Object%20Reference) (OtherComp :type Primitive%20Component%20Object%20Reference) (OtherBodyIndex :type Integer) (bFromSweep :type Boolean) (SweepResult :type Hit%20Result%20Structure%20%28by%20ref%29))
  (Utilities|Casting|CastToBP_Player OtherActor)
  (Input|EnableInput (Game|GetPlayerController 0))
  (bind _returnvalue (UserInterface|CreateWidget "/Game/Characters/Player/Widget/WB_PressE_InTutorial.WB_PressE_InTutorial_C"))
  (bind _output_get (Variables|Default|SetWidget%20REF_0 _returnvalue))
  (UserInterface|Viewport|AddtoViewport _output_get 0))

(event OnComponentEndOverlap(Box)
  (params (OverlappedComponent :type Primitive%20Component%20Object%20Reference) (OtherActor :type Actor%20Object%20Reference) (OtherComp :type Primitive%20Component%20Object%20Reference) (OtherBodyIndex :type Integer))
  (Utilities|Casting|CastToBP_Player OtherActor)
  (Input|DisableInput (Game|GetPlayerController 0))
  (Widget|RemovefromParent (stale OnComponentBeginOverlap(Box) _returnvalue)))

(event Custom|Timer
  (bind _returnvalue (Utilities|Time|SetTimerbyEvent (delegate Custom|Timer) (Variables|Default|GetMaxHoldTime))))

(event Custom|StopTimer
  (Utilities|Time|PauseTimerbyHandle (stale Custom|Timer _returnvalue)))

(event Custom|UpdateTimer
  (bind _widget_ref (Variables|Default|GetWidget%20REF))
  (if (Variables|Default|GetIsHeld?)
    (Variables|/Game/Characters/Player/Widget/WB_Hold.WB_Hold_C|SetTimeHeld _widget_ref (Class|KismetSystemLibrary|GetTimerElapsedTimeHandle (stale Custom|Timer _returnvalue)))
    (Utilities|FlowControl|Delay 0.1)
    (CallFunction|UpdateTimer)
    (else
      (CallFunction|StopTimer)
      (Variables|/Game/Characters/Player/Widget/WB_Hold.WB_Hold_C|SetTimeHeld _widget_ref 0.0))))

(event Input|EnhancedActionEvents|EnhancedInputActionIA_Hold
  (params (ActionValue :type Boolean) (ElapsedSeconds :type Float%20%28double-precision%29) (TriggeredSeconds :type Float%20%28double-precision%29) (InputAction :type Input%20Action%20Object%20Reference :default "/Game/ThirdPerson/Input/Actions/IA_Hold.IA_Hold")))

(event Input|KeyboardEvents|E
  (params (Key :type Key%20Structure))
  (:Pressed
    (Audio|PlaySoundatLocation "/Engine/VREditor/Sounds/UI/Click_on_Button.Click_on_Button" (Transformation|GetWorldLocation (Variables|Default|GetArrow)) "0, 0, 0" 1.0 1.0 0.0 0 0 0 0)
    (Development|SetHiddeninGame (Variables|Default|GetPointLight) false false)
    (Development|SetHiddeninGame (Variables|Default|GetBluelight) true false)
    (Components|DestroyComponent (Variables|Default|GetBox))
    (bind _outactors (Actor|GetAllActorsOfClass "/Game/Maps_Data/LV0_Tutorial/Tutorial/BP_DExitTutorial.BP_DExitTutorial_C"))
    (Default|CollectPoint _outactors)))

(fn ConstructionScript)