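; BP_DEnter_Global is a door Blueprint that slides open and shut as points are collected.
; Each CollectPoint call increments a counter; the first triggers OpenDoor and the second triggers CloseDoor, each guarded by a DoOnce, with later calls doing nothing to the door.
; Separate timelines lerp the door mesh's relative X location for opening and closing, despite their tracks being named DoorRatation.
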(event Custom|Close%20Door
  (bind _door_ratation (Timeline|Timeline Play)
    (:Update
      (Transformation|SetRelativeLocation (Variables|Default|GetDoor) (Math|Vector|MakeVector (Math|Float|Lerp 2.6e+02 -2e+02 _door_ratation) 0.0 0.0) false false))))

(event Custom|Open%20Door
  (bind _door_ratation (Timeline|Open%20Door%20Anim Play)
    (:Update
      (Transformation|SetRelativeLocation (Variables|Default|GetDoor) (Math|Vector|MakeVector (Math|Float|Lerp -2e+02 2.5e+02 _door_ratation) 0.0 0.0) false false))))

(event Custom|CollectPoint
  (Math|Integer|IncrementInt (Variables|Default|GetCollectPointToOpen)
    (:%20%20
      (if (== (Variables|Default|GetCollectPointToOpen) 1)
        (Utilities|FlowControl|DoOnce false
          (:Completed
            (CallFunction|OpenDoor)))
        (elif (== (Variables|Default|GetCollectPointToOpen) 2)
          (Utilities|FlowControl|DoOnce false
            (:Completed
              (CallFunction|CloseDoor))))))))

(fn ConstructionScript)