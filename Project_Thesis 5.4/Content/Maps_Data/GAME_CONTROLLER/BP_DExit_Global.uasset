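; BP_DExit_Global is an exit door that opens once enough points are collected.
; On BeginPlay it finds BP_GameStarter, using its gamemode to set the required count: one for Survival, the configured maximum for Objective.
; CollectPoint increments the count and checks the threshold; Mid Game Objective also requires the game timer to have run out.
; A DoOnce then triggers a timeline that slides the door and plays a metal gate sound.
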(event Custom|Open%20Door
  (bind _door_ratation (Timeline|Open%20Door%20Anim Play)
    (:Update
      (Transformation|SetRelativeLocation (Variables|Default|GetDoor) (Math|Vector|MakeVector (Math|Float|Lerp -2e+02 2.5e+02 _door_ratation) 0.0 0.0) false false))))

(event Custom|CollectPoint
  (Math|Integer|IncrementInt (Variables|Default|GetCollectPointToOpen)
    (:%20%20
      (CallFunction|OpenDoorHandle))))

(event EventBeginPlay
  (bind _returnvalue (Actor|GetActorOfClass "/Game/Maps_Data/GAME_CONTROLLER/BP_GameStarter.BP_GameStarter_C"))
  (Variables|Default|SetGameStarter _returnvalue)
  (bind _foundwidgets (Widget|GetAllWidgetsOfClass "/Game/Maps_Data/GAME_CONTROLLER/WDG_GameStarter.WDG_GameStarter_C" true))
  (Variables|Default|SetGameWidget_Base _foundwidgets)
  (Utilities|FlowControl|Sequence
    (:then_0
      (switch Utilities|FlowControl|Switch|SwitchonEGamemode (Variables|/Game/Maps_Data/GAME_CONTROLLER/BP_GameStarter.BP_GameStarter_C|GetGamemode (Variables|Default|GetGameStarter))
        (:NewEnumerator0
          (Variables|Default|SetMaxCollectPointToOpen 1))
        (:NewEnumerator1
          (Variables|Default|SetMaxCollectPointToOpen (Variables|/Game/Maps_Data/GAME_CONTROLLER/BP_GameStarter.BP_GameStarter_C|GetMax%20Point%20for%20Objective (Variables|Default|GetGameStarter))))))))

(fn ConstructionScript)

(fn OpenDoorHandle
  (bind _gamestarter (Variables|Default|GetGameStarter))
  (if (>= (Variables|Default|GetCollectPointToOpen) (Variables|Default|GetMaxCollectPointToOpen))
    ;[1 1 1] Inbetween Objective
    (switch Utilities|FlowControl|Switch|SwitchonEObjective_Type (Variables|/Game/Maps_Data/GAME_CONTROLLER/BP_GameStarter.BP_GameStarter_C|GetObjective_Type _gamestarter)
      (:NewEnumerator5
        (Utilities|FlowControl|DoOnce false :!label _label
          (:Completed
            (CallFunction|OpenDoor)
            (Audio|PlaySound2D "/Game/Sound/SoundEffect/OpenMetalGate.OpenMetalGate" 1.0 1.0 0.0 0 0))))
      (:NewEnumerator0
        (if (<= (Variables|/Game/Maps_Data/GAME_CONTROLLER/BP_GameStarter.BP_GameStarter_C|GetGameTime_s _gamestarter) 0.0)
          (goto _label)))
      (:NewEnumerator3
        (goto _label)))))