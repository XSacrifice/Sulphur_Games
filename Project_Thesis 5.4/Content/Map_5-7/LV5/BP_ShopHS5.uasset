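; BP_ShopHS5 is a vending-machine shop actor that plays hum and bossa nova sounds at its location on BeginPlay.
; Box overlap with BP_Player enables the actor's input, shows a press-E prompt and opens a Gate; leaving reverses this.
; E runs a FlipFlop: A passes the Gate to open WB_ShopRed with cursor and pawn input disabled.
; B removes the shop, plays a sound and restores game input.
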(event OnComponentBeginOverlap(Box)
  (params (OverlappedComponent :type Primitive%20Component%20Object%20Reference) (OtherActor :type Actor%20Object%20Reference) (OtherComp :type Primitive%20Component%20Object%20Reference) (OtherBodyIndex :type Integer) (bFromSweep :type Boolean) (SweepResult :type Hit%20Result%20Structure%20%28by%20ref%29))
  (bind _returnvalue (Game|GetPlayerController 0))
  (Utilities|Casting|CastToBP_Player OtherActor)
  (Input|EnableInput (Game|GetPlayerController 0))
  (bind _returnvalue_2 (UserInterface|CreateWidget "/Game/ThirdPerson/UI/WB_PressE.WB_PressE_C"))
  (bind _output_get (Variables|Default|SetPress%20E%20Ref _returnvalue_2))
  (UserInterface|Viewport|AddtoViewport _output_get 0)
  (Utilities|FlowControl|Gate true) ; enters at Open
)

(event OnComponentEndOverlap(Box)
  (params (OverlappedComponent :type Primitive%20Component%20Object%20Reference) (OtherActor :type Actor%20Object%20Reference) (OtherComp :type Primitive%20Component%20Object%20Reference) (OtherBodyIndex :type Integer))
  (bind _returnvalue (Game|GetPlayerController 0))
  (Utilities|Casting|CastToBP_Player OtherActor)
  (Input|DisableInput (Game|GetPlayerController 0))
  (Widget|RemovefromParent (stale OnComponentBeginOverlap(Box) _returnvalue_2))
  (Utilities|FlowControl|Gate true) ; enters at Close
)

(event Collision|EventActorBeginOverlap
  (params (OtherActor :type Actor%20Object%20Reference)))

(event EventTick
  (params (DeltaSeconds :type Float%20%28single-precision%29)))

(event EventBeginPlay
  (bind _returnvalue (Transformation|GetActorLocation))
  (Audio|SpawnSoundatLocation "/Game/Sound/SoundEffect/VendingMachine/VendingHum_Cue.VendingHum_Cue" _returnvalue "0, 0, 0" 1.0 1.0 0.0 0 0)
  (Audio|SpawnSoundatLocation "/Game/Sound/SoundEffect/VendingMachine/Bossa_nova_180_BPM_Cue.Bossa_nova_180_BPM_Cue" _returnvalue "0, 0, 0" 1.0 1.0 0.0 0 0))

(event Input|KeyboardEvents|E
  (params (Key :type Key%20Structure))
  (bind _returnvalue (Game|GetPlayerController 0))
  (bind _returnvalue_2 (Game|GetPlayerController 0))
  (:Pressed
    (Utilities|FlowControl|FlipFlop
      (:A
        (Utilities|FlowControl|Gate true
          (:Exit
            (if (not (Variables|Default|GetShopOn))
              (Utilities|FlowControl|Sequence
                (:then_0
                  (Variables|Default|SetShopOn true)
                  (bind _returnvalue_3 (UserInterface|CreateWidget "/Game/Map_Red/WB_ShopRed.WB_ShopRed_C"))
                  (bind _output_get (Variables|Default|SetBuyItemWid _returnvalue_3))
                  (UserInterface|Viewport|AddtoViewport _output_get 0)
                  (Variables|/Script/Engine.PlayerController|SetbShowMouseCursor _returnvalue true)
                  (Input|SetInputModeGameandUI _returnvalue (Variables|Default|GetBuyItemWid) "DoNotLock" true false)
                  (Input|DisableInput (Game|Player|GetPlayerPawn 0) (Game|GetPlayerController 0))))))))
      (:B
        (Audio|PlaySound2D "/Game/Sound/SoundEffect/StickSFX.StickSFX" 1.0 1.0 0.0 0 0)
        (bind _foundwidgets (Widget|GetAllWidgetsOfClass "/Game/Map_Red/WB_ShopRed.WB_ShopRed_C" true))
        (Widget|RemovefromParent _foundwidgets)
        (Variables|/Script/Engine.PlayerController|SetbShowMouseCursor _returnvalue_2 false)
        (Input|SetInputModeGameOnly _returnvalue_2 false)
        (Input|EnableInput (Game|Player|GetPlayerPawn 0) (Game|GetPlayerController 0))
        (Variables|Default|SetShopOn false)))))

(fn ConstructionScript)