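; Exit door actor that opens once enough objective points have been collected.
; On BeginPlay it reads the required count from BP_GameStarter's MaxPointForObjective.
; Each CollectPoint call increments a counter, and reaching the target triggers OpenDoor once with a 2D metal gate sound.
; OpenDoor plays a timeline that slides the Door along relative X, despite its track being named DoorRatation.
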(event Custom|Open%20Door
  (bind _door_ratation (Timeline|Open%20Door%20Anim Play)
    (:Update
      (Transformation|SetRelativeLocation (Variables|Default|GetDoor) (Math|Vector|MakeVector (Math|Float|Lerp -2e+02 2.5e+02 _door_ratation) 0.0 0.0) false false))))

(event Custom|CollectPoint
  (Math|Integer|IncrementInt (Variables|Default|GetCollectPointToOpen)
    (:%20%20
      (if (>= (Variables|Default|GetCollectPointToOpen) (Variables|Default|GetMaxCollectPointToOpen))
        (Utilities|FlowControl|DoOnce false
          (:Completed
            (CallFunction|OpenDoor)
            (Audio|PlaySound2D "/Game/Sound/SoundEffect/OpenMetalGate.OpenMetalGate" 1.0 1.0 0.0 0 0)
            (Utilities|FlowControl|Delay 1.0)))))))

(event EventBeginPlay
  (bind _returnvalue (Actor|GetActorOfClass "/Game/Map_5-7/GAME_CONTROLLER/BP_GameStarter.BP_GameStarter_C"))
  (bind _output_get (Variables|Default|SetGameStarter _returnvalue))
  ;[1 1 1] On Hold (will use in future)
  (Variables|Default|SetMaxCollectPointToOpen (Variables|/Game/Map_5-7/GAME_CONTROLLER/BP_GameStarter.BP_GameStarter_C|GetMax%20Point%20for%20Objective _output_get)))

(fn ConstructionScript)