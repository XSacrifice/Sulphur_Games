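; Freak zombie enemy that melees the player, takes damage and drops loot on death.
; An overlap sphere gates random attack montages, whose short hit window lets the Left collider damage the player.
; Lethal damage spawns scrap and possible pistol ammo, credits quest event 4 if active, then ragdolls the body away from the damage causer before delayed destruction.
; A separate skill-card drop event spawns a smaller scrap reward.
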(event OnComponentBeginOverlap(Sphere)
  (params (OverlappedComponent :type Primitive%20Component%20Object%20Reference) (OtherActor :type Actor%20Object%20Reference) (OtherComp :type Primitive%20Component%20Object%20Reference) (OtherBodyIndex :type Integer) (bFromSweep :type Boolean) (SweepResult :type Hit%20Result%20Structure%20%28by%20ref%29))
  ;[1 1 1] Attack
  (Utilities|Casting|CastToBP_Player OtherActor)
  (Variables|Default|SetZombie%20can%20attack true))

(event OnComponentEndOverlap(Sphere)
  (params (OverlappedComponent :type Primitive%20Component%20Object%20Reference) (OtherActor :type Actor%20Object%20Reference) (OtherComp :type Primitive%20Component%20Object%20Reference) (OtherBodyIndex :type Integer))
  ;[1 1 1] Attack
  (Utilities|Casting|CastToBP_Player OtherActor)
  (Variables|Default|SetZombie%20can%20attack false))

(event OnComponentBeginOverlap(Left)
  (params (OverlappedComponent :type Primitive%20Component%20Object%20Reference) (OtherActor :type Actor%20Object%20Reference) (OtherComp :type Primitive%20Component%20Object%20Reference) (OtherBodyIndex :type Integer) (bFromSweep :type Boolean) (SweepResult :type Hit%20Result%20Structure%20%28by%20ref%29))
  ;[1 1 1] Attack
  (Utilities|Casting|CastToBP_Player OtherActor)
  (Utilities|FlowControl|DoOnce false :!label _label
    (:Completed
      (CallFunction|Hit)
      (goto _label Reset))))

(event Custom|Droploot%20SkillCard
  (bind _returnvalue (Transformation|GetActorLocation))
  ;[1 1 1] Drop Loot (Skill)
  (Variables|Default|SetIsDropped? true)
  (Game|SpawnActorfromClass "/Game/Shop/Scrap/BP_SScrap.BP_SScrap_C" (Math|Conversions|ToTransform(Vector) (- _returnvalue "0.000000,0.000000,100.000000")) "AlwaysSpawn" "MultiplyWithRoot" 0 0)
  (bind _outhit (Collision|LineTraceByChannel _returnvalue (- _returnvalue "0.000000,0.000000,200.000000") "TraceTypeQuery1" false (Utilities|Array|MakeArray (Game|GetPlayerCharacter 0)) "None"))
  (Game|SpawnActorfromClass (Utilities|Select :Index (Math|Random|RandomInteger 5) :Option%200 "/Game/Shop/Scrap/BP_SScrap.BP_SScrap_C" :Option%201 0 :Option%202 0 :Option%203 0 :Option%204 0) (Math|Transform|MakeTransform (.Location (Collision|BreakHitResult _outhit)) (Math|Rotator|MakeRotator 0.0 0.0 (Math|Random|RandomFloatinRange 0.0 3.6e+02))) "AlwaysSpawn" "MultiplyWithRoot" 0 0))

(event Custom|Attack
  ;[1 1 1] Attack
  (if (not (Variables|Default|GetIs%20Dead?))
    (Utilities|FlowControl|DoOnce false :!label _label
      (:Completed
        (Animation|PlayAnimMontage (.OutItem (Utilities|Array|Random (Variables|Default|GetAttack%20Animation%20Montage))) 1.0 "None")
        (Variables|Default|SetHit? true)
        (Utilities|FlowControl|Delay 0.5)
        (Audio|PlaySoundatLocation "/Game/Sound/Human/Cue/ZBite.ZBite" (Transformation|GetActorLocation) "0, 0, 0" 1.0 1.0 0.0 "/Game/MilitaryWeapDark/Sound/Knife/Zombieshot_SA.Zombieshot_SA" 0 0 0)
        (Variables|Default|SetHit? false)
        (goto _label Reset)))))

(event Custom|Hit
  ;[1 1 1] Attack
  (if (not (Variables|Default|GetIs%20Dead?))
    (if (Variables|Default|GetHit?)
      (Game|Damage|ApplyDamage (Variables|Default|GetAs%20BP%20Third%20Person%20Character) (Variables|Default|GetFreak%20Damage) 0 self)
      (Default|PlayerGotDamage (Variables|Default|GetAs%20BP%20Third%20Person%20Character)))))

(event Custom|DropLoot
  (bind _returnvalue (Transformation|GetActorLocation))
  (bind _returnvalue_2 (- _returnvalue "0.000000,0.000000,100.000000"))
  (bind _returnvalue_3 (Math|Conversions|ToTransform(Vector) _returnvalue_2))
  ;[1 1 1] Drop Loot
  (Variables|Default|SetIsDropped? true)
  (Game|SpawnActorfromClass "/Game/Shop/Scrap/BP_SScrap.BP_SScrap_C" _returnvalue_3 "AlwaysSpawn" "MultiplyWithRoot" 0 0)
  (Game|SpawnActorfromClass "/Game/Shop/Scrap/BP_SScrap.BP_SScrap_C" _returnvalue_3 "AlwaysSpawn" "MultiplyWithRoot" 0 0)
  (Game|SpawnActorfromClass "/Game/Shop/Scrap/BP_SScrap.BP_SScrap_C" _returnvalue_3 "AlwaysSpawn" "MultiplyWithRoot" 0 0)
  (bind _outhit (Collision|LineTraceByChannel _returnvalue (- _returnvalue "0.000000,0.000000,200.000000") "TraceTypeQuery1" false (Utilities|Array|MakeArray (Game|GetPlayerCharacter 0)) "None"))
  (Game|SpawnActorfromClass (Utilities|Select :Index (Math|Random|RandomInteger 8) :Option%200 "/Game/ThirdPerson/Blueprints/Item/BP_PistolAmmoPickuup_3.BP_PistolAmmoPickuup_3_C" :Option%201 0 :Option%202 0 :Option%203 0 :Option%204 0 :Option%205 0 :Option%206 0 :Option%207 0 :Option%208 0) (Math|Transform|MakeTransform (.Location (Collision|BreakHitResult _outhit)) (Math|Rotator|MakeRotator 0.0 0.0 (Math|Random|RandomFloatinRange 0.0 3.6e+02))) "AlwaysSpawn" "MultiplyWithRoot" 0 0)
  (bind _asbp_player (Utilities|Casting|CastToBP_Player (Game|GetPlayerCharacter 0)))
  (Utilities|FlowControl|Sequence
    (:then_1
      (if (Variables|/Game/Characters/Player/Blueprint/BP_Player.BP_Player_C|GetEventPointNo4? _asbp_player)
        (bind _outactors (Actor|GetAllActorsOfClass "/Game/EventQuest/Quest_4/BP_QuestEvent_4.BP_QuestEvent_4_C"))
        (Default|CollectPointZombie _outactors)))))

(event Custom|check%20attack
  ;[1 1 1] Attack
  (if (Variables|Default|GetZombie%20can%20attack)
    (CallFunction|Attack)))

(event EventBeginPlay
  ;[1 1 1] Begin Play
  (bind _asbp_player (Utilities|Casting|CastToBP_Player (Game|GetPlayerCharacter 0)))
  (Variables|Default|SetAs%20BP%20Third%20Person%20Character _asbp_player)
  (Variables|Default|SetEnemyHealth (Variables|Default|GetMax%20Health)))

(fn ConstructionScript)

(event Game|Damage|EventAnyDamage
  (params (Damage :type Float%20%28single-precision%29) (DamageType :type Damage%20Type%20Object%20Reference) (InstigatedBy :type Controller%20Object%20Reference) (DamageCauser :type Actor%20Object%20Reference))
  (bind _mesh (Variables|Character|GetMesh))
  ;[1 1 1] On Any Damage
  (Variables|Default|SetDamage%20Causer DamageCauser)
  (Audio|PlaySoundatLocation "/Game/MilitaryWeapDark/Sound/Shotgun/Shotgun_ImpactBody_Cue.Shotgun_ImpactBody_Cue" (Transformation|GetActorLocation) "0, 0, 0" 1.0 1.0 0.0 "/Game/MilitaryWeapDark/Sound/Knife/Zombieshot_SA.Zombieshot_SA" 0 0 0)
  (bind _output_get (Variables|Default|SetEnemyHealth (- (Variables|Default|GetEnemyHealth) Damage)))
  (if (<= _output_get 0.0)
    (if (Variables|Default|GetIs%20Dead?)
      (Variables|Default|SetIsDropped? true)
      (else
        (Audio|PlaySoundatLocation "/Game/Sound/Human/BigZombieDeath.BigZombieDeath" (Transformation|GetActorLocation) "0, 0, 0" 1.0 1.0 0.0 "/Game/MilitaryWeapDark/Sound/Knife/Zombieshot_SA.Zombieshot_SA" 0 0 0)))
    (for _index (range 0 (Math|Random|RandomInteger 2))
      (if (not (Variables|Default|GetIs%20Dead?))
        (if (not (Variables|Default|GetIsDropped?))
          (CallFunction|DropLoot))))
    (Pawn|Components|CharacterMovement|DisableMovement (Variables|Character|GetCharacterMovement))
    (Variables|Default|SetIs%20Dead? true)
    (Physics|SetSimulatePhysics _mesh true)
    (Physics|AddImpulse _mesh (* (Math|Vector|Normalize (- (Transformation|GetActorLocation) (Transformation|GetActorLocation (Variables|Default|GetDamage%20Causer)))) 500) "None" true)
    (Collision|SetCollisionResponsetoChannel (Variables|Character|GetMesh) "ECC_Visibility" "ECR_Ignore")
    (Collision|SetCollisionResponsetoChannel (Variables|Character|GetMesh) "ECC_Pawn" "ECR_Ignore")
    (Utilities|FlowControl|Delay 8.0)
    (Actor|DestroyActor)
    (elif (not (Variables|Default|GetIs%20Dead?))
      (Audio|PlaySoundatLocation "/Game/Sound/Human/Cue/BIGZGruntCue.BIGZGruntCue" (Transformation|GetActorLocation) "0, 0, 0" 1.0 1.0 0.0 "/Game/MilitaryWeapDark/Sound/Knife/Zombieshot_SA.Zombieshot_SA" 0 0 0))))