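; BP_Walker is the walker zombie enemy, with randomized health, melee attacks, loot drops and a shove that launches other walkers.
; Sphere overlaps enable attacking and start timer-driven turning toward the player, while attack montages open a brief window for two hand hitboxes to deal damage.
; Taking damage can trigger a stagger.
; Death drops scrap, credits active quest events and skill-card bonus loot, then ragdolls the body before destroying it.
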(event OnComponentBeginOverlap(Sphere)
  (params (OverlappedComponent :type Primitive%20Component%20Object%20Reference) (OtherActor :type Actor%20Object%20Reference) (OtherComp :type Primitive%20Component%20Object%20Reference) (OtherBodyIndex :type Integer) (bFromSweep :type Boolean) (SweepResult :type Hit%20Result%20Structure%20%28by%20ref%29))
  ;[1 1 1] Player Check
  (bind _asbp_player (Utilities|Casting|CastToBP_Player OtherActor))
  (Variables|Default|SetChaREF _asbp_player)
  (Variables|Default|SetZombie%20can%20Attack? true))

(event OnComponentEndOverlap(Sphere)
  (params (OverlappedComponent :type Primitive%20Component%20Object%20Reference) (OtherActor :type Actor%20Object%20Reference) (OtherComp :type Primitive%20Component%20Object%20Reference) (OtherBodyIndex :type Integer))
  ;[1 1 1] Player Check
  (Utilities|Casting|CastToBP_Player OtherActor)
  (Variables|Default|SetZombie%20can%20Attack? false))

(event OnComponentBeginOverlap(BoxR)
  (params (OverlappedComponent :type Primitive%20Component%20Object%20Reference) (OtherActor :type Actor%20Object%20Reference) (OtherComp :type Primitive%20Component%20Object%20Reference) (OtherBodyIndex :type Integer) (bFromSweep :type Boolean) (SweepResult :type Hit%20Result%20Structure%20%28by%20ref%29))
  ;[1 1 1] Hand Hitbox
  (Utilities|Casting|CastToBP_Player OtherActor)
  (Utilities|FlowControl|DoOnce false :!label _label
    (:Completed
      (if (Variables|Default|GetHit?)
        (Variables|Default|SethandR true)
        (Collision|SetCollisionEnabled (Variables|Default|GetBoxL) "NoCollision")
        (CallFunction|Hit)
        (Utilities|FlowControl|Delay 1.0)
        (Variables|Default|SethandR false)
        (goto _label Reset)))))

(event OnComponentBeginOverlap(BoxL)
  (params (OverlappedComponent :type Primitive%20Component%20Object%20Reference) (OtherActor :type Actor%20Object%20Reference) (OtherComp :type Primitive%20Component%20Object%20Reference) (OtherBodyIndex :type Integer) (bFromSweep :type Boolean) (SweepResult :type Hit%20Result%20Structure%20%28by%20ref%29))
  ;[1 1 1] Hand Hitbox
  (Utilities|Casting|CastToBP_Player OtherActor)
  (Utilities|FlowControl|DoOnce false :!label _label
    (:Completed
      (if (Variables|Default|GetHit?)
        (Variables|Default|SethandL true)
        (Collision|SetCollisionEnabled (Variables|Default|GetBoxR) "NoCollision")
        (CallFunction|HitL)
        (Utilities|FlowControl|Delay 1.0)
        (Variables|Default|SethandL false)
        (goto _label Reset)))))

(event OnComponentHit(CapsuleComponent)
  (params (HitComponent :type Primitive%20Component%20Object%20Reference) (OtherActor :type Actor%20Object%20Reference) (OtherComp :type Primitive%20Component%20Object%20Reference) (NormalImpulse :type Vector :default "0, 0, 0") (Hit :type Hit%20Result%20Structure%20%28by%20ref%29))
  (bind _asbp_player (Utilities|Casting|CastToBP_Player OtherActor))
  (if (not (Variables|/Game/Characters/Player/Blueprint/BP_Player.BP_Player_C|GetisDead? _asbp_player))
    (Physics|SetSimulatePhysics (Variables|Collision|GetCapsuleComponent) true)
    (Utilities|FlowControl|Delay 5.0)
    (Physics|SetSimulatePhysics (Variables|Collision|GetCapsuleComponent) false)))

(event OnComponentBeginOverlap(Sphere2)
  (params (OverlappedComponent :type Primitive%20Component%20Object%20Reference) (OtherActor :type Actor%20Object%20Reference) (OtherComp :type Primitive%20Component%20Object%20Reference) (OtherBodyIndex :type Integer) (bFromSweep :type Boolean) (SweepResult :type Hit%20Result%20Structure%20%28by%20ref%29))
  ;[1 1 1] Look
  (bind _asbp_player (Utilities|Casting|CastToBP_Player OtherActor))
  (Variables|Default|SetChaREF _asbp_player)
  (bind _returnvalue (Utilities|Time|SetTimerbyEvent (delegate Custom|Rotate) 0.01 true))
  (Variables|Default|SetTimeHandle _returnvalue))

(event Custom|FollowPlayer)

(event Custom|Droploot%20SkillCard
  (bind _returnvalue (Math|Random|RandomInteger 2))
  (bind _returnvalue_2 (Transformation|GetActorLocation))
  ;[1 1 1] Drop System
  ;;[1 1 1] Upgrade
  (Variables|Default|SetIs%20Dropped? true)
  (bind _outhit (Collision|LineTraceByChannel _returnvalue_2 (- _returnvalue_2 "0.000000,0.000000,200.000000") "TraceTypeQuery1" false (Utilities|Array|MakeArray (Game|GetPlayerCharacter 0)) "None"))
  (Game|SpawnActorfromClass (Utilities|Select :Index _returnvalue :Option%200 "/Game/Shop/Scrap/BP_SScrap.BP_SScrap_C" :Option%201 0 :Option%202 0) (Math|Transform|MakeTransform (.Location (Collision|BreakHitResult _outhit)) (Math|Rotator|MakeRotator 0.0 0.0 (Math|Random|RandomFloatinRange 0.0 3.6e+02))) "AlwaysSpawn" "MultiplyWithRoot" 0 0)
  (if (== _returnvalue 0)
    (Audio|SpawnSoundatLocation "/Game/Sound/SoundEffect/VendingMachine/CoinSpill_Cue.CoinSpill_Cue" (Transformation|GetActorLocation) "0, 0, 0" 1.0 1.0 0.0 0 0)))

(event Custom|Look)

(event Custom|StopLogic
  (bind _self self)
  (bind _returnvalue (AI|GetAIController _self))
  (bind _braincomponent (Variables|/Script/AIModule.AIController|GetBrainComponent _returnvalue))
  ;[1 1 1] push
  (AI|Logic|StopLogic _braincomponent "")
  (Utilities|FlowControl|Delay 2.0)
  (Class|BrainComponent|RestartLogic _braincomponent))

(event Custom|Attack
  ;[1 1 1] Attack
  (if (not (Variables|Default|GetIsDead))
    (Collision|SetCollisionEnabled (Variables|Default|GetBoxL) "QueryOnly")
    (Collision|SetCollisionEnabled (Variables|Default|GetBoxR) "QueryOnly")
    (Utilities|FlowControl|DoOnce false :!label _label
      (:Completed
        (Animation|PlayAnimMontage (.OutItem (Utilities|Array|Random (Variables|Default|GetAttack%20Anim))) 1.0 "None")
        (Variables|Default|SetHit? true)
        (Utilities|FlowControl|Delay 0.5)
        (Audio|PlaySoundatLocation "/Game/Sound/Human/Cue/ZBite.ZBite" (Transformation|GetActorLocation) "0, 0, 0" 1.0 1.0 0.0 "/Game/MilitaryWeapDark/Sound/Knife/Zombieshot_SA.Zombieshot_SA" 0 0 0)
        (Variables|Default|SetHit? false)
        (Collision|SetCollisionEnabled (Variables|Default|GetBoxL) "NoCollision")
        (Collision|SetCollisionEnabled (Variables|Default|GetBoxR) "NoCollision")
        (goto _label Reset)))))

(event Custom|hitL
  ;[1 1 1] Hit Damage
  (if (not (Variables|Default|GetIsDead))
    (if (Variables|Default|GetHit?)
      (if (Variables|Default|GethandL)
        (Game|Damage|ApplyDamage (Variables|Default|GetAs%20BP%20Third%20Person%20Character) 1e+01 0 self)
        (Variables|Default|SetDamaged_L true)
        (Utilities|FlowControl|Delay 0.2)
        (Variables|Default|SetDamaged_L false)))))

(event Custom|DropLoot
  (bind _returnvalue (Transformation|GetActorLocation))
  ;[1 1 1] Drop System
  (Variables|Default|SetIs%20Dropped? true)
  (Game|SpawnActorfromClass "/Game/Shop/Scrap/BP_SScrap.BP_SScrap_C" (Math|Conversions|ToTransform(Vector) (- _returnvalue "0.000000,0.000000,100.000000")) "AlwaysSpawn" "MultiplyWithRoot" 0 0)
  (bind _outhit (Collision|LineTraceByChannel _returnvalue (- _returnvalue "0.000000,0.000000,200.000000") "TraceTypeQuery1" false (Utilities|Array|MakeArray (Game|GetPlayerCharacter 0)) "None"))
  (Game|SpawnActorfromClass (Utilities|Select :Index (Math|Random|RandomInteger 12) :Option%200 "/Game/Shop/Scrap/BP_MScrap.BP_MScrap_C" :Option%201 0 :Option%202 0 :Option%203 0 :Option%204 0 :Option%205 0 :Option%206 0 :Option%207 0 :Option%208 0 :Option%209 0 :Option%2010 0 :Option%2011 0 :Option%2012 0) (Math|Transform|MakeTransform (.Location (Collision|BreakHitResult _outhit)) (Math|Rotator|MakeRotator 0.0 0.0 (Math|Random|RandomFloatinRange 0.0 3.6e+02))) "AlwaysSpawn" "MultiplyWithRoot" 0 0))

(event Custom|AnyPush)

(event Custom|check%20player
  ;[1 1 1] Player Check
  (if (Variables|Default|GetZombie%20can%20Attack?)
    (CallFunction|Attack)))

(event Custom|PushedAndPush
  (bind _arrow1 (Variables|Default|GetArrow1))
  (bind _arrow1_2 (Variables|Default|GetArrow1))
  (bind _returnvalue (Transformation|GetWorldLocation _arrow1))
  (bind _returnvalue_2 (Transformation|GetWorldRotation _arrow1_2))
  (bind _returnvalue_3 (Math|Vector|GetForwardVector _returnvalue_2))
  (bind _returnvalue_4 (* _returnvalue_3 8e+02))
  ;[1 1 1] push
  (bind _outhits (Collision|MultiSphereTraceForObjects _returnvalue (+ _returnvalue (* (Math|Vector|GetForwardVector (Transformation|GetWorldRotation _arrow1)) 6e+01)) 4e+01 (Utilities|Array|MakeArray "ObjectTypeQuery3") false 0 "ForDuration" true "(R=1.000000,G=0.000000,B=0.000000,A=1.000000)" "(R=0.000000,G=1.000000,B=0.000000,A=1.000000)" 0.2))
  (for _array_element _outhits
    (bind _asbp_walker (Utilities|Casting|CastToBP_Walker (.HitActor (Collision|BreakHitResult _array_element))))
    (CallFunction|StopLogic)
    (Pawn|Components|CharacterMovement|DisableMovement (Variables|/Script/Engine.Character|GetCharacterMovement _asbp_walker))
    (Pawn|Components|CharacterMovement|SetMovementMode (Variables|/Script/Engine.Character|GetCharacterMovement _asbp_walker) "MOVE_Flying" 0)
    (Development|PrintString "pushing" true true "(R=0.038695,G=1.000000,B=0.000000,A=1.000000)")
    (Utilities|FlowControl|Delay 0.1)
    (Character|LaunchCharacter _asbp_walker (Math|Vector|MakeVector (.x _returnvalue_4) (.y _returnvalue_4) (+ (.z _returnvalue_4) 3e+01)) false false)
    (Variables|Default|SetPushed true)
    (Development|PrintString "pushed")
    (Utilities|FlowControl|Delay 0.5)
    (Pawn|Components|CharacterMovement|SetMovementMode (Variables|/Script/Engine.Character|GetCharacterMovement _asbp_walker) "MOVE_Walking" 0)
    (Development|PrintString "walk")
    (Variables|Default|SetPushed false)))

(event Custom|Hit
  ;[1 1 1] Hit Damage
  (if (not (Variables|Default|GetIsDead))
    (if (Variables|Default|GetHit?)
      (if (Variables|Default|GethandR)
        (Game|Damage|ApplyDamage (Variables|Default|GetAs%20BP%20Third%20Person%20Character) 1e+01 0 self)
        (Variables|Default|SetDamaged_R true)
        (Utilities|FlowControl|Delay 0.2)
        (Variables|Default|SetDamaged_R false)))))

(event Custom|Rotate
  ;[1 1 1] Look
  (Transformation|SetActorRotation (Math|Rotator|MakeRotator 0.0 0.0 (.yaw (Math|Interpolation|RInterpTo (Transformation|GetActorRotation) (Math|Rotator|FindLookatRotation (Transformation|GetActorLocation) (Transformation|GetActorLocation (Variables|Default|GetChaREF))) (Utilities|Time|GetWorldDeltaSeconds) 1.0)))))

(event EventBeginPlay
  ;[1 1 1] Game Start
  (bind _asbp_player (Utilities|Casting|CastToBP_Player (Game|GetPlayerCharacter 0)))
  (Variables|Default|SetAs%20BP%20Third%20Person%20Character _asbp_player)
  (Variables|Default|SetWalker_MaxHealth (Math|Random|RandomIntegerinRange 41 43))
  (Variables|Default|SetWalker_CurrentHealth (Variables|Default|GetWalker_MaxHealth)))

(event Collision|EventActorBeginOverlap
  (params (OtherActor :type Actor%20Object%20Reference)))

(event EventTick
  (params (DeltaSeconds :type Float%20%28single-precision%29)))

(fn ConstructionScript)

(event Game|Damage|EventAnyDamage
  (params (Damage :type Float%20%28single-precision%29) (DamageType :type Damage%20Type%20Object%20Reference) (InstigatedBy :type Controller%20Object%20Reference) (DamageCauser :type Actor%20Object%20Reference))
  (bind _mesh (Variables|Character|GetMesh))
  (Variables|Default|SetDamage%20Causer DamageCauser)
  (Audio|PlaySoundatLocation "/Game/MilitaryWeapDark/Sound/Shotgun/Shotgun_ImpactBody_Cue.Shotgun_ImpactBody_Cue" (Transformation|GetActorLocation) "0, 0, 0" 1.0 1.0 0.0 "/Game/MilitaryWeapDark/Sound/Knife/Zombieshot_SA.Zombieshot_SA" 0 0 0)
  (bind _output_get (Variables|Default|SetWalker_CurrentHealth (- (Variables|Default|GetWalker_CurrentHealth) Damage)))
  (if (<= _output_get 0.0)
    (if (Variables|Default|GetIsDead)
      (Variables|Default|SetIs%20Dropped? true)
      (else
        (Audio|PlaySoundatLocation "/Game/Sound/Human/BigZombieDeath.BigZombieDeath" (Transformation|GetActorLocation) "0, 0, 0" 1.0 1.0 0.0 "/Game/MilitaryWeapDark/Sound/Knife/Zombieshot_SA.Zombieshot_SA" 0 0 0)))
    (for _index (range 0 (Math|Random|RandomInteger 2))
      (if (not (Variables|Default|GetIsDead))
        (if (not (Variables|Default|GetIs%20Dropped?))
          (bind _asbp_player (Utilities|Casting|CastToBP_Player (Game|GetPlayerCharacter 0)))
          (CallFunction|DropLoot)
          (Utilities|FlowControl|Sequence
            (:then_0
              (if (Variables|/Game/Characters/Player/Blueprint/BP_Player.BP_Player_C|GetEventPoint? _asbp_player)
                (bind _outactors (Actor|GetAllActorsOfClass "/Game/EventQuest/Quest_1/BP_QuestEvent.BP_QuestEvent_C"))
                (Default|CollectPointZombie _outactors)))
            (:then_1
              (if (Variables|/Game/Characters/Player/Blueprint/BP_Player.BP_Player_C|GetHave%20Shot? _asbp_player)
                (if (Variables|/Game/Characters/Player/Blueprint/BP_Player.BP_Player_C|GetSkill%20Card%20+1%20Scrap%20Drop _asbp_player)
                  (CallFunction|DroplootSkillCard))))
            (:then_2
              (if (Variables|/Game/Characters/Player/Blueprint/BP_Player.BP_Player_C|GetEventPointNo2? _asbp_player)
                (bind _outactors_2 (Actor|GetAllActorsOfClass "/Game/EventQuest/Quest_2/BP_QuestEvent_2.BP_QuestEvent_2_C"))
                (Default|CollectPointZombie _outactors_2)))
            (:then_3
              (if (Variables|/Game/Characters/Player/Blueprint/BP_Player.BP_Player_C|GetEventPointNo3? _asbp_player)
                (bind _outactors_3 (Actor|GetAllActorsOfClass "/Game/EventQuest/Quest_3/BP_QuestEvent_3.BP_QuestEvent_3_C"))
                (Default|CollectPointZombie _outactors_3)))
            (:then_4
              (if (Variables|/Game/Characters/Player/Blueprint/BP_Player.BP_Player_C|GetEventPointNo4? _asbp_player)
                (bind _outactors_4 (Actor|GetAllActorsOfClass "/Game/EventQuest/Quest_4/BP_QuestEvent_4.BP_QuestEvent_4_C"))
                (Default|CollectPointZombie _outactors_4)))))))
    (Pawn|Components|CharacterMovement|DisableMovement (Variables|Character|GetCharacterMovement))
    (Variables|Default|SetIsDead true)
    (Physics|SetSimulatePhysics _mesh true)
    (Physics|AddImpulse _mesh (* (Math|Vector|Normalize (- (Transformation|GetActorLocation) (Transformation|GetActorLocation (Variables|Default|GetDamage%20Causer)))) 500) "None" true)
    (Collision|SetCollisionResponsetoChannel (Variables|Character|GetMesh) "ECC_Visibility" "ECR_Ignore")
    (Collision|SetCollisionResponsetoChannel (Variables|Character|GetMesh) "ECC_Pawn" "ECR_Ignore")
    (Utilities|FlowControl|Delay 8.0)
    (Actor|DestroyActor)
    (else
      (|StunSystem)
      (Audio|PlaySoundatLocation "/Game/Sound/Human/Cue/SZGruntCue.SZGruntCue" (Transformation|GetActorLocation) "0, 0, 0" 1.0 1.0 0.0 "/Game/MilitaryWeapDark/Sound/Knife/Zombieshot_SA.Zombieshot_SA" 0 0 0))))