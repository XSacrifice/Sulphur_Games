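; BP_Runner is a zombie enemy with randomized health that melees the player and drops loot when killed.
; A proximity sphere gates checkplayer's montage attack, which briefly arms left and right hand boxes that deal damage on overlap.
; Non-lethal hits randomly trigger a movement-stopping stagger.
; Death spawns scrap and possible pickups, credits active quest events, then ragdolls the body away from the damage causer before destroying it.
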(event OnComponentBeginOverlap(Sphere)
  (params (OverlappedComponent :type Primitive%20Component%20Object%20Reference) (OtherActor :type Actor%20Object%20Reference) (OtherComp :type Primitive%20Component%20Object%20Reference) (OtherBodyIndex :type Integer) (bFromSweep :type Boolean) (SweepResult :type Hit%20Result%20Structure%20%28by%20ref%29))
  ;[1 1 1] Comment
  (Utilities|Casting|CastToBP_Player OtherActor)
  (Variables|Default|SetZombie%20Can%20Attack true))

(event OnComponentEndOverlap(Sphere)
  (params (OverlappedComponent :type Primitive%20Component%20Object%20Reference) (OtherActor :type Actor%20Object%20Reference) (OtherComp :type Primitive%20Component%20Object%20Reference) (OtherBodyIndex :type Integer))
  ;[1 1 1] Comment
  (Utilities|Casting|CastToBP_Player OtherActor)
  (Variables|Default|SetZombie%20Can%20Attack false))

(event OnComponentBeginOverlap(BoxL)
  (params (OverlappedComponent :type Primitive%20Component%20Object%20Reference) (OtherActor :type Actor%20Object%20Reference) (OtherComp :type Primitive%20Component%20Object%20Reference) (OtherBodyIndex :type Integer) (bFromSweep :type Boolean) (SweepResult :type Hit%20Result%20Structure%20%28by%20ref%29))
  ;[1 1 1] Comment
  (Utilities|Casting|CastToBP_Player OtherActor)
  (Development|PrintString "L")
  (if (Variables|Default|GetHit?)
    (Variables|Default|SetHandL true)
    (CallFunction|HitL)
    (Utilities|FlowControl|Delay 1.0)
    (Variables|Default|SetHandL false)))

(event OnComponentBeginOverlap(BoxR)
  (params (OverlappedComponent :type Primitive%20Component%20Object%20Reference) (OtherActor :type Actor%20Object%20Reference) (OtherComp :type Primitive%20Component%20Object%20Reference) (OtherBodyIndex :type Integer) (bFromSweep :type Boolean) (SweepResult :type Hit%20Result%20Structure%20%28by%20ref%29))
  ;[1 1 1] Comment
  (Utilities|Casting|CastToBP_Player OtherActor)
  (Development|PrintString "R")
  (if (Variables|Default|GetHit?)
    (Variables|Default|SetHandR true)
    (CallFunction|Hit)
    (Utilities|FlowControl|Delay 1.0)
    (Variables|Default|SetHandR false)))

(event Custom|FollowPlayer)

(event Custom|Droploot%20SkillCard
  (bind _returnvalue (Transformation|GetActorLocation))
  ;[1 1 1] Comment
  ;;[1 1 1] Comment
  (Variables|Default|SetIsDropped? true)
  (Game|SpawnActorfromClass "/Game/Shop/Scrap/BP_SScrap.BP_SScrap_C" (Math|Conversions|ToTransform(Vector) (- _returnvalue "0.000000,0.000000,100.000000")) "AlwaysSpawn" "MultiplyWithRoot" 0 0)
  (bind _outhit (Collision|LineTraceByChannel _returnvalue (- _returnvalue "0.000000,0.000000,200.000000") "TraceTypeQuery1" false (Utilities|Array|MakeArray (Game|GetPlayerCharacter 0)) "None"))
  (Game|SpawnActorfromClass (Utilities|Select :Index (Math|Random|RandomInteger 5) :Option%200 "/Game/Shop/Scrap/BP_SScrap.BP_SScrap_C" :Option%201 0 :Option%202 0 :Option%203 0 :Option%204 0) (Math|Transform|MakeTransform (.Location (Collision|BreakHitResult _outhit)) (Math|Rotator|MakeRotator 0.0 0.0 (Math|Random|RandomFloatinRange 0.0 3.6e+02))) "AlwaysSpawn" "MultiplyWithRoot" 0 0))

(event Custom|DropLoot
  (bind _returnvalue (Transformation|GetActorLocation))
  (bind _returnvalue_2 (- _returnvalue "0.000000,0.000000,100.000000"))
  (bind _returnvalue_3 (Math|Conversions|ToTransform(Vector) _returnvalue_2))
  ;[1 1 1] Comment
  ;;[1 1 1] Comment
  (Variables|Default|SetIsDropped? true)
  (Game|SpawnActorfromClass "/Game/Shop/Scrap/BP_SScrap.BP_SScrap_C" _returnvalue_3 "AlwaysSpawn" "MultiplyWithRoot" 0 0)
  (Game|SpawnActorfromClass "/Game/Shop/Scrap/BP_SScrap.BP_SScrap_C" _returnvalue_3 "AlwaysSpawn" "MultiplyWithRoot" 0 0)
  (bind _outhit (Collision|LineTraceByChannel _returnvalue (- _returnvalue "0.000000,0.000000,200.000000") "TraceTypeQuery1" false (Utilities|Array|MakeArray (Game|GetPlayerCharacter 0)) "None"))
  (Game|SpawnActorfromClass (Utilities|Select :Index (Math|Random|RandomInteger 8) :Option%200 "/Game/ThirdPerson/Blueprints/Item/BP_PistolAmmoPickuup_3.BP_PistolAmmoPickuup_3_C" :Option%201 0 :Option%202 0 :Option%203 0 :Option%204 0 :Option%205 0 :Option%206 0 :Option%207 0 :Option%208 0) (Math|Transform|MakeTransform (.Location (Collision|BreakHitResult _outhit)) (Math|Rotator|MakeRotator 0.0 0.0 (Math|Random|RandomFloatinRange 0.0 3.6e+02))) "AlwaysSpawn" "MultiplyWithRoot" 0 0))

(event Custom|hitL
  ;[1 1 1] Comment
  (if (not (Variables|Default|GetIsDead?))
    (if (not (Variables|Default|GetDamaged_R))
      (if (Variables|Default|GetHit?)
        (if (Variables|Default|GetHandL)
          (Game|Damage|ApplyDamage (Variables|Default|GetAs%20BP%20Third%20Person%20Character) 3.0 0 self)
          (Variables|Default|SetDamaged_L true)
          (Utilities|FlowControl|Delay 0.2)
          (Variables|Default|SetDamaged_L false)
          (Collision|SetCollisionEnabled (Variables|Default|GetBoxL) "NoCollision"))))))

(event Custom|Hit
  ;[1 1 1] Comment
  (if (not (Variables|Default|GetIsDead?))
    (if (not (Variables|Default|GetDamaged_L))
      (if (Variables|Default|GetHit?)
        (if (Variables|Default|GetHandR)
          (Game|Damage|ApplyDamage (Variables|Default|GetAs%20BP%20Third%20Person%20Character) 3.0 0 self)
          (Variables|Default|SetDamaged_R true)
          (Utilities|FlowControl|Delay 0.2)
          (Variables|Default|SetDamaged_R false)
          (Collision|SetCollisionEnabled (Variables|Default|GetBoxR) "NoCollision"))))))

(event Custom|Attack
  ;[1 1 1] Comment
  (if (not (Variables|Default|GetIsDead?))
    (Utilities|FlowControl|DoOnce false :!label _label
      (:Completed
        (Animation|PlayAnimMontage (Variables|Default|GetAttack%20Animation%20Montage_1) 1.0 "None")
        (Collision|SetCollisionEnabled (Variables|Default|GetBoxR) "QueryOnly")
        (Variables|Default|SetHit? true)
        (Utilities|FlowControl|Delay 0.5)
        (Audio|PlaySoundatLocation "/Game/Sound/Human/Cue/ZBite.ZBite" (Transformation|GetActorLocation) "0, 0, 0" 1.0 1.0 0.0 "/Game/MilitaryWeapDark/Sound/Knife/Zombieshot_SA.Zombieshot_SA" 0 0 0)
        (Utilities|FlowControl|Delay 2.0)
        (Variables|Default|SetHit? false)
        (goto _label Reset)))))

(event Custom|check%20player
  ;[1 1 1] Comment
  (if (Variables|Default|GetZombie%20Can%20Attack)
    (CallFunction|Attack)))

(event Custom|test%20Hit
  (if (not (Variables|Default|GetIsDead?))
    (if (Variables|Default|GetHit?)
      (Game|Damage|ApplyDamage (Variables|Default|GetAs%20BP%20Third%20Person%20Character) 3.0 0 self))))

(event EventBeginPlay
  ;[1 1 1] แ
  (bind _asbp_player (Utilities|Casting|CastToBP_Player (Game|GetPlayerCharacter 0)))
  (Variables|Default|SetAs%20BP%20Third%20Person%20Character _asbp_player)
  (Variables|Default|SetEnemyMaxHealth (Math|Random|RandomIntegerinRange 21 41))
  (Variables|Default|SetEnemyHealth (Variables|Default|GetEnemyMaxHealth))
  (Collision|SetCollisionEnabled (Variables|Default|GetBoxR) "NoCollision"))

(event Collision|EventActorBeginOverlap
  (params (OtherActor :type Actor%20Object%20Reference)))

(event EventTick
  (params (DeltaSeconds :type Float%20%28single-precision%29)))

(fn ConstructionScript)

(event Game|Damage|EventAnyDamage
  (params (Damage :type Float%20%28single-precision%29) (DamageType :type Damage%20Type%20Object%20Reference) (InstigatedBy :type Controller%20Object%20Reference) (DamageCauser :type Actor%20Object%20Reference))
  (bind _mesh (Variables|Character|GetMesh))
  (Variables|Default|SetDamage%20Causer DamageCauser)
  (Audio|PlaySoundatLocation "/Game/MilitaryWeapDark/Sound/Shotgun/Shotgun_ImpactBody_Cue.Shotgun_ImpactBody_Cue" (Transformation|GetActorLocation) "0, 0, 0" 1.0 1.0 0.0 "/Game/MilitaryWeapDark/Sound/Knife/Zombieshot_SA.Zombieshot_SA" 0 0 0)
  (bind _output_get (Variables|Default|SetEnemyHealth (- (Variables|Default|GetEnemyHealth) Damage)))
  (if (<= _output_get 0.0)
    (if (Variables|Default|GetIsDead?)
      (Variables|Default|SetIsDropped? true)
      (else
        (Audio|PlaySoundatLocation "/Game/Sound/Human/BigZombieDeath.BigZombieDeath" (Transformation|GetActorLocation) "0, 0, 0" 1.0 1.0 0.0 "/Game/MilitaryWeapDark/Sound/Knife/Zombieshot_SA.Zombieshot_SA" 0 0 0)))
    (for _index (range 0 (Math|Random|RandomInteger 2))
      (if (not (Variables|Default|GetIsDead?))
        (if (not (Variables|Default|GetIsDropped?))
          (bind _asbp_player (Utilities|Casting|CastToBP_Player (Game|GetPlayerCharacter 0)))
          (CallFunction|DropLoot)
          (Utilities|FlowControl|Sequence
            (:then_0
              (if (Variables|/Game/Characters/Player/Blueprint/BP_Player.BP_Player_C|GetEventPointNo3? _asbp_player)
                (bind _outactors (Actor|GetAllActorsOfClass "/Game/EventQuest/Quest_3/BP_QuestEvent_3.BP_QuestEvent_3_C"))
                (Default|CollectPointZombie _outactors)))
            (:then_1
              (if (Variables|/Game/Characters/Player/Blueprint/BP_Player.BP_Player_C|GetEventPointNo4? _asbp_player)
                (bind _outactors_2 (Actor|GetAllActorsOfClass "/Game/EventQuest/Quest_4/BP_QuestEvent_4.BP_QuestEvent_4_C"))
                (Default|CollectPointZombie _outactors_2)))))))
    (Pawn|Components|CharacterMovement|DisableMovement (Variables|Character|GetCharacterMovement))
    (Variables|Default|SetIsDead? true)
    (Physics|SetSimulatePhysics _mesh true)
    (Physics|AddImpulse _mesh (* (Math|Vector|Normalize (- (Transformation|GetActorLocation) (Transformation|GetActorLocation (Variables|Default|GetDamage%20Causer)))) 500) "None" true)
    (Collision|SetCollisionResponsetoChannel (Variables|Character|GetMesh) "ECC_Visibility" "ECR_Ignore")
    (Collision|SetCollisionResponsetoChannel (Variables|Character|GetMesh) "ECC_Pawn" "ECR_Ignore")
    (Utilities|FlowControl|Delay 5.0)
    (Actor|DestroyActor)
    (else
      (|StunSystem)
      (Audio|PlaySoundatLocation "/Game/Sound/Human/Cue/SZGruntCue.SZGruntCue" (Transformation|GetActorLocation) "0, 0, 0" 1.0 1.0 0.0 "/Game/MilitaryWeapDark/Sound/Knife/Zombieshot_SA.Zombieshot_SA" 0 0 0))))