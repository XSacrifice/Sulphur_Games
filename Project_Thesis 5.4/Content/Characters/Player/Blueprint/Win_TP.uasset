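; Win_TP is a win trigger that ends the run when the player pawn overlaps its box.
; It fades the camera, then calls the player's ResetInstance, carries half the prior currency over, bumps the win streak and saves through the game instance.
; It then shows the WB_Win widget with UI-only mouse input and plays the end jingle.
; A branch to stop the Mastermind music is left unconnected.
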(event OnComponentBeginOverlap(Box)
  (params (OverlappedComponent :type Primitive%20Component%20Object%20Reference) (OtherActor :type Actor%20Object%20Reference) (OtherComp :type Primitive%20Component%20Object%20Reference) (OtherBodyIndex :type Integer) (bFromSweep :type Boolean) (SweepResult :type Hit%20Result%20Structure%20%28by%20ref%29))
  (bind _returnvalue (Game|GetPlayerController 0))
  (if (== OtherActor (Game|Player|GetPlayerPawn 0))
    (CameraFades|StartCameraFade :self (Game|GetPlayerCameraManager 0) :ToAlpha 1.0 :Duration 1.0)
    (Utilities|FlowControl|Delay 1.0)
    (Utilities|FlowControl|Sequence
      (:then_1
        (bind _ascurrent_instance (Utilities|Casting|CastToCurrent_Instance (Game|GetGameInstance)))
        (bind _output_get (Variables|/Game/Characters/Player/Blueprint/Current_Instance.Current_Instance_C|SetBonus%20Currency%20Inst _ascurrent_instance (/ (Variables|/Game/Characters/Player/Blueprint/Current_Instance.Current_Instance_C|GetCurrency%20inst _ascurrent_instance) 2)))
        (bind _asbp_player (Utilities|Casting|CastToBP_Player (Game|Player|GetPlayerPawn 0)))
        (Default|ResetInstance _asbp_player)
        (Variables|/Game/Characters/Player/Blueprint/Current_Instance.Current_Instance_C|SetCurrency%20inst _ascurrent_instance _output_get)
        (bind _result (Math|Integer|IncrementInt (Variables|/Game/Characters/Player/Blueprint/Current_Instance.Current_Instance_C|GetWin%20Streak _ascurrent_instance))
          (:%20%20
            (Variables|/Game/Characters/Player/Blueprint/Current_Instance.Current_Instance_C|SetWin%20Streak _ascurrent_instance _result)
            (Default|SaveGame _ascurrent_instance)
            (bind _returnvalue_2 (UserInterface|CreateWidget "/Game/Characters/Player/Blueprint/Widget/WB_Win.WB_Win_C"))
            (UserInterface|Viewport|AddtoViewport _returnvalue_2 0)
            (Variables|/Script/Engine.PlayerController|SetbShowMouseCursor _returnvalue true)
            (Input|SetInputModeUIOnly _returnvalue _returnvalue_2 "DoNotLock" false)
            (bind _returnvalue_3 (Audio|SpawnSound2D "/Game/Sound/Music/End_Jingle.End_Jingle" 1.0 1.0 0.0 0))
            (Variables|Default|SetEnd%20Jingle%20Ref _returnvalue_3)))))))

(fn ConstructionScript)