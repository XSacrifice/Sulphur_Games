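; TestNewLevel1 is a trigger actor that moves the player to another level when their pawn overlaps its Box.
; The overlap fades the camera out, waits for the fade, then shows the WDG_LoadingScreen widget.
; It then stores TeleTag and LevelName in the Current_Instance game instance, calls GameSaveInstance on the BP_Player cached at BeginPlay, and opens the level by name.
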(event OnComponentBeginOverlap(Box)
  (params (OverlappedComponent :type Primitive%20Component%20Object%20Reference) (OtherActor :type Actor%20Object%20Reference) (OtherComp :type Primitive%20Component%20Object%20Reference) (OtherBodyIndex :type Integer) (bFromSweep :type Boolean) (SweepResult :type Hit%20Result%20Structure%20%28by%20ref%29))
  (if (== OtherActor (Game|Player|GetPlayerPawn 0))
    (CameraFades|StartCameraFade :self (Game|GetPlayerCameraManager 0) :ToAlpha 1.0 :Duration 1.0)
    (Utilities|FlowControl|Delay 1.0)
    (bind _returnvalue (UserInterface|CreateWidget "/Game/Characters/Player/Widget/WDG_LoadingScreen.WDG_LoadingScreen_C"))
    (UserInterface|Viewport|AddtoViewport _returnvalue 0)
    (Utilities|FlowControl|Sequence
      (:then_0
        (bind _ascurrent_instance (Utilities|Casting|CastToCurrent_Instance (Game|GetGameInstance)))
        (Variables|/Game/Current_Instance.Current_Instance_C|SetLevel%20Tag%20inst _ascurrent_instance (Variables|Default|GetTele%20Tag))
        (Variables|/Game/Current_Instance.Current_Instance_C|SetLevel%20Inst _ascurrent_instance (Variables|Default|GetLevel%20Name)))
      (:then_1
        (Default|GameSaveInstance (Variables|Default|GetAs%20BP%20Player)))
      (:then_2
        (Game|OpenLevel(byName) (Variables|Default|GetLevel%20Name))))))

(event EventBeginPlay
  (bind _asbp_player (Utilities|Casting|CastToBP_Player (Game|GetPlayerCharacter 0)))
  (Variables|Default|SetAs%20BP%20Player _asbp_player))

(fn ConstructionScript)