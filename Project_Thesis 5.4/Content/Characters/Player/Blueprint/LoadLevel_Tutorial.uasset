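; LoadLevel_Tutorial is a trigger volume that moves the player to another level when their pawn enters its Box.
; On overlap it fades the camera out, waits for the fade, then shows the WDG_LoadingScreen widget.
; It stores TeleTag in the Current_Instance game instance, calls ResetInstance on BP_Player, and opens the level named by LevelName.
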(event OnComponentBeginOverlap(Box)
  (params (OverlappedComponent :type Primitive%20Component%20Object%20Reference) (OtherActor :type Actor%20Object%20Reference) (OtherComp :type Primitive%20Component%20Object%20Reference) (OtherBodyIndex :type Integer) (bFromSweep :type Boolean) (SweepResult :type Hit%20Result%20Structure%20%28by%20ref%29))
  (if (== OtherActor (Game|Player|GetPlayerPawn 0))
    (CameraFades|StartCameraFade :self (Game|GetPlayerCameraManager 0) :ToAlpha 1.0 :Duration 1.0)
    (Utilities|FlowControl|Delay 1.0)
    (bind _returnvalue (UserInterface|CreateWidget "/Game/Characters/Player/Widget/WDG_LoadingScreen.WDG_LoadingScreen_C"))
    (UserInterface|Viewport|AddtoViewport _returnvalue 0)
    (bind _ascurrent_instance (Utilities|Casting|CastToCurrent_Instance (Game|GetGameInstance)))
    (Variables|/Game/Current_Instance.Current_Instance_C|SetLevel%20Tag%20inst _ascurrent_instance (Variables|Default|GetTeleTag))
    (bind _asbp_player (Utilities|Casting|CastToBP_Player (Game|GetPlayerCharacter 0)))
    (Default|ResetInstance _asbp_player)
    (Game|OpenLevel(byName) (Variables|Default|GetLevelName))))

(fn ConstructionScript)