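; Current_Instance persists the player's death counter and win streak through a save slot.
; SaveGame writes both values into a fresh BP_Save object as BodyCount and PlayerRank, saves it to PlayerSaveSlot and prints a debug message.
; LoadGame copies them back if that slot exists and casts to BP_Save; a missing slot leaves the current values untouched.
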(fn SaveGame
  (bind _returnvalue (SaveGame|CreateSaveGameObject "/Game/Characters/Player/Blueprint/BP_Save.BP_Save_C"))
  (Variables|/Game/Characters/Player/Blueprint/BP_Save.BP_Save_C|SetBodyCount _returnvalue (Variables|Default|GetDeath%20Counter))
  (Variables|/Game/Characters/Player/Blueprint/BP_Save.BP_Save_C|SetPlayerRank _returnvalue (Variables|Default|GetWin%20Streak))
  (SaveGame|SaveGametoSlot _returnvalue "PlayerSaveSlot")
  (Development|PrintString "Save Create"))

(fn LoadGame
  (bind _returnvalue (SaveGame|DoesSaveGameExist "PlayerSaveSlot"))
  (if _returnvalue
    (bind _returnvalue_2 (SaveGame|LoadGamefromSlot "PlayerSaveSlot"))
    (bind _asbp_save (Utilities|Casting|CastToBP_Save _returnvalue_2))
    (Variables|Default|SetDeath%20Counter (Variables|/Game/Characters/Player/Blueprint/BP_Save.BP_Save_C|GetBodyCount _asbp_save))
    (Variables|Default|SetWin%20Streak (Variables|/Game/Characters/Player/Blueprint/BP_Save.BP_Save_C|GetPlayerRank _asbp_save))))