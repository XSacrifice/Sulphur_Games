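; BP_DEnterRed is a door actor in the red map that opens once enough collect points have been registered.
; Each CollectPoint call increments a counter, and reaching the maximum fires OpenDoor a single time through a DoOnce.
; OpenDoor plays a timeline that slides the door along its relative X axis, and the actor destroys itself one second later.
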(event Custom|Open%20Door
  (bind _door_ratation (Timeline|Open%20Door%20Anim Play)
    (:Update
      (Transformation|SetRelativeLocation (Variables|Default|GetDoor) (Math|Vector|MakeVector (Math|Float|Lerp -2e+02 2.5e+02 _door_ratation) 0.0 0.0) false false))))

(event Custom|CollectPoint
  (Math|Integer|IncrementInt (Variables|Default|GetCollectPointToOpen)
    (:%20%20
      (if (>= (Variables|Default|GetCollectPointToOpen) (Variables|Default|GetMaxCollectPointToOpen))
        (Utilities|FlowControl|DoOnce false
          (:Completed
            (CallFunction|OpenDoor)
            (Utilities|FlowControl|Delay 1.0)
            (Actor|DestroyActor)))))))

(fn ConstructionScript)