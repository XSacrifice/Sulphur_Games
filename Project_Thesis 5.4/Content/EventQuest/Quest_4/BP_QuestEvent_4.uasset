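; Quest event actor for quest 4, a point-zombie collection objective that rewards a coupon.
; Its start event notifies BP_Player and shows a MasterMind dialogue widget, then adds the quest widget after a short delay.
; Each collect event increments a counter; at the maximum it increments the player's coupons, copies the total to the game instance, plays a sound, clears the quest flag and widget, and destroys itself.
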(event Custom|PointZombies_Event_4
  (bind _returnvalue (Actor|GetActorOfClass "/Game/Characters/Player/Blueprint/BP_Player.BP_Player_C"))
  (Default|PointZombie4EventStart _returnvalue)
  (bind _returnvalue_2 (UserInterface|CreateWidget "/Game/EventQuest/Quest_4/WB_DialogueMasterMindPointZom_4.WB_DialogueMasterMindPointZom_4_C"))
  (UserInterface|Viewport|AddtoViewport _returnvalue_2 0)
  (Utilities|FlowControl|Delay 3.0)
  (bind _returnvalue_3 (UserInterface|CreateWidget "/Game/EventQuest/Quest_4/WB_Quest_4.WB_Quest_4_C"))
  (UserInterface|Viewport|AddtoViewport _returnvalue_3 0))

(event Custom|CollectPointZombie
  (bind _result (Math|Integer|IncrementInt (Variables|Default|GetCollectPointZom))
    (:%20%20
      (Development|PrintString (Utilities|String|ToString(Integer) _result))
      (if (>= (Variables|Default|GetCollectPointZom) (Variables|Default|GetMaxCollectPointZom))
        (bind _returnvalue (Actor|GetActorOfClass "/Game/Characters/Player/Blueprint/BP_Player.BP_Player_C"))
        (Development|PrintString "+1Coupon")
        (bind _output_get (Variables|/Game/Characters/Player/Blueprint/BP_Player.BP_Player_C|SetCoupon _returnvalue (+ (Variables|/Game/Characters/Player/Blueprint/BP_Player.BP_Player_C|GetCoupon _returnvalue) 1)))
        (bind _ascurrent_instance (Utilities|Casting|CastToCurrent_Instance (Game|GetGameInstance)))
        (Variables|/Game/Characters/Player/Blueprint/Current_Instance.Current_Instance_C|SetCoupon%20Inst _ascurrent_instance _output_get)
        (Audio|PlaySound2D "/Game/EventQuest/Quest_1/PassQuest_sound.PassQuest_sound" 1.0 1.0 0.0 0 0)
        (Variables|/Game/Characters/Player/Blueprint/BP_Player.BP_Player_C|SetEventPointNo4? _returnvalue false)
        (bind _foundwidgets (Widget|GetAllWidgetsOfClass "/Game/EventQuest/Quest_4/WB_Quest_4.WB_Quest_4_C" true))
        (Widget|RemovefromParent _foundwidgets)
        (Actor|DestroyActor)))))

(event EventTick
  (params (DeltaSeconds :type Float%20%28single-precision%29)))

(event Collision|EventActorBeginOverlap
  (params (OtherActor :type Actor%20Object%20Reference)))

(event EventBeginPlay)

(fn ConstructionScript)