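; BP_QuestEvent is a quest actor that runs the first quest, a zombie point collection event.
; PointZombies_Event notifies BP_Player, shows the mastermind dialogue, then adds the quest widget after a short delay.
; CollectPointZombie counts pickups; at the maximum it awards a medkit saved to the game instance, plays a sound, clears the player's event flag, removes the widget and destroys itself.
; Several disconnected leftover nodes never run.
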(event Custom|PointZombies_Event
  (bind _returnvalue (Actor|GetActorOfClass "/Game/Characters_Added/Player/BP_Player.BP_Player_C"))
  (Default|PointZombieEventStart _returnvalue)
  (bind _returnvalue_2 (UserInterface|CreateWidget "/Game/EventQuest/Quest_1/WB_DialogueMasterMindPointZom.WB_DialogueMasterMindPointZom_C"))
  (UserInterface|Viewport|AddtoViewport _returnvalue_2 0)
  (Utilities|FlowControl|Delay 2.0)
  (bind _returnvalue_3 (UserInterface|CreateWidget "/Game/EventQuest/Quest_1/WB_Quest1.WB_Quest1_C"))
  (UserInterface|Viewport|AddtoViewport _returnvalue_3 0))

(event Custom|CollectPointZombie
  (bind _result (Math|Integer|IncrementInt (Variables|Default|GetCollectPointZom))
    (:%20%20
      (Development|PrintString (Utilities|String|ToString(Integer) _result))
      (if (>= (Variables|Default|GetCollectPointZom) (Variables|Default|GetMaxCollectPointZom))
        (bind _returnvalue (Actor|GetActorOfClass "/Game/Characters_Added/Player/BP_Player.BP_Player_C"))
        (Development|PrintString "Medkit +1")
        (Variables|/Game/Characters_Added/Player/BP_Player.BP_Player_C|SetHealthPickup _returnvalue (+ (Variables|/Game/Characters_Added/Player/BP_Player.BP_Player_C|GetHealthPickup _returnvalue) 1))
        (Default|UpdateHealthPickup _returnvalue)
        (bind _ascurrent_instance (Utilities|Casting|CastToCurrent_Instance (Game|GetGameInstance)))
        (Variables|/Game/Current_Instance.Current_Instance_C|SetHealthPickup%20inst _ascurrent_instance (Variables|/Game/Characters_Added/Player/BP_Player.BP_Player_C|GetHealthPickup _returnvalue))
        (Audio|PlaySound2D "/Game/EventQuest/Quest_1/PassQuest_sound.PassQuest_sound" 1.0 1.0 0.0 0 0)
        (Variables|/Game/Characters_Added/Player/BP_Player.BP_Player_C|SetEventPoint? _returnvalue false)
        (bind _foundwidgets (Widget|GetAllWidgetsOfClass "/Game/EventQuest/Quest_1/WB_Quest1.WB_Quest1_C" true))
        (Widget|RemovefromParent _foundwidgets)
        (Actor|DestroyActor)))))

(event EventTick
  (params (DeltaSeconds :type Float%20%28single-precision%29)))

(event Collision|EventActorBeginOverlap
  (params (OtherActor :type Actor%20Object%20Reference)))

(event EventBeginPlay)

(fn ConstructionScript)