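; Tutorial trigger for Room1 that shows the WB_TalkwithBotton dialogue widget the first time its box is overlapped.
; On overlap it switches to UI-only input with a cursor, disables pawn input, sets Start, destroys itself and calls SpawnObjective on ObjectiveSpawnerRef.
; A T key handler gated by Start removes the widget and restores game input, although the actor is already destroyed when Start becomes true.
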(event OnComponentBeginOverlap(Box)
  (params (OverlappedComponent :type Primitive%20Component%20Object%20Reference) (OtherActor :type Actor%20Object%20Reference) (OtherComp :type Primitive%20Component%20Object%20Reference) (OtherBodyIndex :type Integer) (bFromSweep :type Boolean) (SweepResult :type Hit%20Result%20Structure%20%28by%20ref%29))
  (bind _returnvalue (Game|GetPlayerController 0))
  (Utilities|FlowControl|DoOnce false
    (:Completed
      (bind _returnvalue_2 (UserInterface|CreateWidget "/Game/Map_Tutorial/Room1/WB_TalkwithBotton.WB_TalkwithBotton_C"))
      (UserInterface|Viewport|AddtoViewport _returnvalue_2 0)
      (Variables|/Script/Engine.PlayerController|SetbShowMouseCursor _returnvalue true)
      (Input|SetInputModeUIOnly _returnvalue (Variables|Default|Gettutorial) "DoNotLock" false)
      (Input|DisableInput (Game|Player|GetPlayerPawn 0) (Game|GetPlayerController 0))
      (Variables|Default|Setstart true)
      (Actor|DestroyActor)
      (Game|SetGamePaused false)
      (Development|PrintString "Hello")
      (Default|SpawnObjective (Variables|Default|GetObjectiveSpawnerRef)))))

(event EventBeginPlay)

(event Collision|EventActorBeginOverlap
  (params (OtherActor :type Actor%20Object%20Reference)))

(event EventTick
  (params (DeltaSeconds :type Float%20%28single-precision%29)))

(event Input|KeyboardEvents|T
  (params (Key :type Key%20Structure :default "None"))
  (bind _returnvalue (Game|GetPlayerController 0))
  (:Pressed
    (if (Variables|Default|Getstart)
      (bind _foundwidgets (Widget|GetAllWidgetsOfClass "/Game/Map_Tutorial/Room1/WB_TalkwithBotton.WB_TalkwithBotton_C" true))
      (Widget|RemovefromParent _foundwidgets)
      (Variables|/Script/Engine.PlayerController|SetbShowMouseCursor _returnvalue false)
      (Input|SetInputModeGameOnly _returnvalue false)
      (Input|EnableInput (Game|Player|GetPlayerPawn 0) (Game|GetPlayerController 0)))))

(fn ConstructionScript)