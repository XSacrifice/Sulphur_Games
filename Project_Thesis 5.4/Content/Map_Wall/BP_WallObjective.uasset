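; Wall objective the player completes by holding IA_Hold inside its Box trigger, with a valve-turning sound.
; Player overlap enables input, shows the WB_Hold widget and opens a gate for the hold input.
; A retriggerable delay checks the input is still held, then swaps lights, destroys the Box and calls CollectPoint on BP_DExitWall actors.
; A timer polled by a recursive delay loop feeds hold progress to the widget.
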(event OnComponentBeginOverlap(Box)
  (params (OverlappedComponent :type Primitive%20Component%20Object%20Reference) (OtherActor :type Actor%20Object%20Reference) (OtherComp :type Primitive%20Component%20Object%20Reference) (OtherBodyIndex :type Integer) (bFromSweep :type Boolean) (SweepResult :type Hit%20Result%20Structure%20%28by%20ref%29))
  (Utilities|Casting|CastToBP_Player OtherActor)
  (Input|EnableInput (Game|GetPlayerController 0))
  (bind _returnvalue (UserInterface|CreateWidget "/Game/ThirdPerson/UI/WB_Hold.WB_Hold_C"))
  (bind _output_get (Variables|Default|SetWidget%20REF _returnvalue))
  (UserInterface|Viewport|AddtoViewport _output_get 0)
  (Variables|/Game/ThirdPerson/UI/WB_Hold.WB_Hold_C|SetMaxTimeHeld _output_get (Variables|Default|GetMaxHoldTime))
  (Utilities|FlowControl|Gate true) ; enters at Open
)

(event OnComponentEndOverlap(Box)
  (params (OverlappedComponent :type Primitive%20Component%20Object%20Reference) (OtherActor :type Actor%20Object%20Reference) (OtherComp :type Primitive%20Component%20Object%20Reference) (OtherBodyIndex :type Integer))
  (Utilities|Casting|CastToBP_Player OtherActor)
  (Input|DisableInput (Game|GetPlayerController 0))
  (Widget|RemovefromParent (stale OnComponentBeginOverlap(Box) _returnvalue))
  (Utilities|FlowControl|Gate true) ; enters at Close
)

(event Custom|Timer
  (bind _returnvalue (Utilities|Time|SetTimerbyEvent (delegate Custom|Timer) (Variables|Default|GetMaxHoldTime))))

(event Custom|StopTimer
  (Utilities|Time|PauseTimerbyHandle (stale Custom|Timer _returnvalue)))

(event Custom|UpdateTimer
  (bind _widget_ref (Variables|Default|GetWidget%20REF))
  (if (Variables|Default|GetIsHeld?)
    (Variables|/Game/ThirdPerson/UI/WB_Hold.WB_Hold_C|SetTimeHeld _widget_ref (Class|KismetSystemLibrary|GetTimerElapsedTimeHandle (stale Custom|Timer _returnvalue)))
    (Utilities|FlowControl|Delay 0.1)
    (CallFunction|UpdateTimer)
    (else
      (CallFunction|StopTimer)
      (Variables|/Game/ThirdPerson/UI/WB_Hold.WB_Hold_C|SetTimeHeld _widget_ref 0.0))))

(event Input|EnhancedActionEvents|EnhancedInputActionIA_Hold
  (params (ActionValue :type Boolean) (ElapsedSeconds :type Float%20%28double-precision%29) (TriggeredSeconds :type Float%20%28double-precision%29) (InputAction :type Input%20Action%20Object%20Reference :default "/Game/ThirdPerson/Input/Actions/IA_Hold.IA_Hold"))
  (:Triggered
    (Variables|Default|SetIsHeld? true)
    (Audio|PlaySound2D "/Game/Sound/SoundEffect/ValveTurningOnce.ValveTurningOnce" 1.0 1.0 0.0 0 0)
    (Utilities|FlowControl|Gate true
      (:Exit
        (Utilities|FlowControl|Sequence
          (:then_0
            (Utilities|FlowControl|RetriggerableDelay (Variables|Default|GetMaxHoldTime))
            (if (Variables|Default|GetIsHeld?)
              (Development|SetHiddeninGame (Variables|Default|GetPointLight) false false)
              (Development|SetHiddeninGame (Variables|Default|GetBluelight) true false)
              (Components|DestroyComponent (Variables|Default|GetBox))
              (bind _outactors (Actor|GetAllActorsOfClass "/Game/Map_Wall/BP_DExitWall.BP_DExitWall_C"))
              (Default|CollectPoint _outactors)))
          (:then_1
            (CallFunction|Timer)
            (CallFunction|UpdateTimer))))))
  (:Completed
    (Variables|Default|SetIsHeld? false)))

(fn ConstructionScript)