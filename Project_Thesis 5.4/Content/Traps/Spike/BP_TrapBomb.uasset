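; BP_TrapBomb is a one-shot bomb trap that explodes when a BP_Player or BP_Walker overlaps its Box.
; Either overlap applies slight damage to player character 0, even when a walker triggers it, then plays an explosion sound, fires the RadialForce impulse and destroys the actor.
; Radial damage, the explosion particle and spike-trap logic with timed flag resets are leftover, unconnected nodes.
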(event OnComponentBeginOverlap(Box)
  (params (OverlappedComponent :type Primitive%20Component%20Object%20Reference) (OtherActor :type Actor%20Object%20Reference) (OtherComp :type Primitive%20Component%20Object%20Reference) (OtherBodyIndex :type Integer) (bFromSweep :type Boolean) (SweepResult :type Hit%20Result%20Structure%20%28by%20ref%29))
  (Utilities|FlowControl|Sequence
    (:then_0
      (Utilities|Casting|CastToBP_Player OtherActor)
      (Game|Damage|ApplyDamage (Game|GetPlayerCharacter 0) (Math|Random|RandomFloatinRange 0.1 0.1) 0 self)
      (Audio|PlaySoundatLocation "/Game/StarterContent/Audio/Explosion_Cue.Explosion_Cue" (Transformation|GetActorLocation) "0, 0, 0" 1.0 1.0 0.0 0 0 0 0)
      (Class|RadialForceComponent|FireImpulse (Variables|Default|GetRadialForce))
      (Actor|DestroyActor))
    (:then_1
      (Utilities|Casting|CastToBP_Walker OtherActor)
      (Game|Damage|ApplyDamage (Game|GetPlayerCharacter 0) (Math|Random|RandomFloatinRange 0.1 0.1) 0 self)
      (Audio|PlaySoundatLocation "/Game/StarterContent/Audio/Explosion_Cue.Explosion_Cue" (Transformation|GetActorLocation) "0, 0, 0" 1.0 1.0 0.0 0 0 0 0)
      (Class|RadialForceComponent|FireImpulse (Variables|Default|GetRadialForce))
      (Actor|DestroyActor))))

(event Custom|CustomEvent
  (Variables|Default|SetIsTriggered? false)
  (Variables|Default|SetSpikeUp false))

(event Custom|ResetPls
  (Variables|Default|SetIsTriggered? false)
  (Variables|Default|SetSpikeUp false))

(event EventBeginPlay)

(fn ConstructionScript)