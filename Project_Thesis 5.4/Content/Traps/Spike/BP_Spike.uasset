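; BP_Spike is a spike trap that damages the player when they overlap its collision.
; An overlap by BP_Player, if not already triggered, sets SpikeUp, applies fixed damage to player character 0 and plays a 2D sound.
; A one-second timer then calls ResetPls to clear both flags and re-arm the trap.
; A similar BP_Walker damage branch is left disconnected and never runs.
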(event OnComponentBeginOverlap(Collision)
  (params (OverlappedComponent :type Primitive%20Component%20Object%20Reference) (OtherActor :type Actor%20Object%20Reference) (OtherComp :type Primitive%20Component%20Object%20Reference) (OtherBodyIndex :type Integer) (bFromSweep :type Boolean) (SweepResult :type Hit%20Result%20Structure%20%28by%20ref%29))
  (Utilities|FlowControl|Sequence
    (:then_0
      (Utilities|Casting|CastToBP_Player OtherActor)
      (if (not (Variables|Default|GetIsTriggered?))
        (Variables|Default|SetIsTriggered? true)
        (Variables|Default|SetSpikeUp true)
        (Game|Damage|ApplyDamage (Game|GetPlayerCharacter 0) (Math|Random|RandomFloatinRange 5.0 5.0) 0 self)
        (Utilities|Time|SetTimerbyEvent (delegate Custom|ResetPls) 1.0)
        (Audio|PlaySound2D "/Game/Traps/Spike/SpikeSE.SpikeSE" 1.0 1.0 0.0 0 0)))))

(event Custom|CustomEvent
  (Variables|Default|SetIsTriggered? false)
  (Variables|Default|SetSpikeUp false))

(event Custom|ResetPls
  (Variables|Default|SetIsTriggered? false)
  (Variables|Default|SetSpikeUp false))

(event EventBeginPlay)

(event Collision|EventActorBeginOverlap
  (params (OtherActor :type Actor%20Object%20Reference)))

(event EventTick
  (params (DeltaSeconds :type Float%20%28single-precision%29)))

(fn ConstructionScript)