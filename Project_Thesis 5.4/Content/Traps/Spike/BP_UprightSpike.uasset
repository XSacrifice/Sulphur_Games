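; BP_UprightSpike is a spike trap that damages the player on contact.
; The spike plays a hide idle animation at start.
; When BP_Player overlaps Collision, it plays the trap animation, damages player character 0 and plays a sound, with IsTriggered blocking retriggers until a short delay clears it.
; Unconnected leftover nodes hold an unused BP_Walker cast, enemy damage and timer-based resets.
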(event OnComponentBeginOverlap(Collision)
  (params (OverlappedComponent :type Primitive%20Component%20Object%20Reference) (OtherActor :type Actor%20Object%20Reference) (OtherComp :type Primitive%20Component%20Object%20Reference) (OtherBodyIndex :type Integer) (bFromSweep :type Boolean) (SweepResult :type Hit%20Result%20Structure%20%28by%20ref%29))
  (Utilities|Casting|CastToBP_Player OtherActor)
  (if (not (Variables|Default|GetIsTriggered?))
    (Variables|Default|SetIsTriggered? true)
    (Variables|Default|SetSpikeUp true)
    (Components|Animation|PlayAnimation (Variables|Default|GetSpike) "/Game/Traps/Spike/SpikeTrap_HideAnimation_Anim.SpikeTrap_HideAnimation_Anim" false)
    (Game|Damage|ApplyDamage (Game|GetPlayerCharacter 0) (Math|Random|RandomFloatinRange 15.0 15.0) 0 self)
    (Audio|PlaySoundatLocation "/Game/Traps/Spike/SpikeCue.SpikeCue" (Transformation|GetActorLocation) "0, 0, 0" 1.0 1.0 0.0 0 0 0 0)
    (Utilities|FlowControl|Delay 0.5)
    (Variables|Default|SetIsTriggered? false)
    (Variables|Default|SetSpikeUp false)))

(event Custom|CustomEvent
  (Variables|Default|SetIsTriggered? false)
  (Variables|Default|SetSpikeUp false))

(event Custom|ResetPls
  (Variables|Default|SetIsTriggered? false)
  (Variables|Default|SetSpikeUp false))

(event Collision|EventActorBeginOverlap
  (params (OtherActor :type Actor%20Object%20Reference)))

(event EventTick
  (params (DeltaSeconds :type Float%20%28single-precision%29)))

(event EventBeginPlay
  (Components|Animation|PlayAnimation (Variables|Default|GetSpike) "/Game/Traps/Spike/SpikeTrap_HideAnimation_Idle.SpikeTrap_HideAnimation_Idle" false))

(fn ConstructionScript)