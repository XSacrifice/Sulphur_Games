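; Explosive fire extinguisher trap that reacts to damage with a fuse or an immediate blast.
; Damage lowers its health; at zero the fuse sound stops and it explodes, otherwise the fuse plays and it explodes after a short delay.
; The blast loops a random number of times, applying radial damage, effects, sound and a physics impulse before destroying the actor.
; Incoming radial damage destroys it directly with only an explosion particle.
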(event Game|Damage|EventRadialDamage
  (params (DamageReceived :type Float%20%28single-precision%29) (DamageType :type Damage%20Type%20Object%20Reference) (Origin :type Vector :default "0, 0, 0") (HitInfo :type Hit%20Result%20Structure%20%28by%20ref%29) (InstigatedBy :type Controller%20Object%20Reference) (DamageCauser :type Actor%20Object%20Reference))
  (Actor|DestroyActor)
  (Effects|SpawnEmitteratLocation "/Game/StarterContent/Particles/P_Explosion.P_Explosion" (Transformation|GetActorLocation) "0, 0, 0" "3.000000,3.000000,3.000000"))

(event Game|Damage|EventAnyDamage
  (params (Damage :type Float%20%28single-precision%29) (DamageType :type Damage%20Type%20Object%20Reference) (InstigatedBy :type Controller%20Object%20Reference) (DamageCauser :type Actor%20Object%20Reference))
  (bind _output_get (Variables|Default|SetBarrelHealth (- (Variables|Default|GetBarrelHealth) Damage)))
  (if (<= _output_get 0.0)
    (Audio|Components|Audio|Stop (Variables|Default|GetFuzeRef))
    (for _index (range 0 (Math|Random|RandomInteger 2)) :!label _label
      (Game|Damage|ApplyRadialDamage 2e+01 (Transformation|GetActorLocation) 5e+02 0 0 self 0 false "ECC_Visibility")
      (Effects|SpawnEmitteratLocation "/Game/StarterContent/Particles/P_Explosion.P_Explosion" (Transformation|GetActorLocation) "0, 0, 0" "3.000000,3.000000,3.000000")
      (Audio|PlaySoundatLocation "/Game/Sound/SoundEffect/Audio/Explosion_Cue.Explosion_Cue" (Transformation|GetActorLocation) "0, 0, 0" 1.0 1.0 0.0 0 0 0 0)
      (Class|RadialForceComponent|FireImpulse (Variables|Default|GetRadialForce)))
    (Actor|DestroyActor)
    (else
      (bind _returnvalue (Audio|SpawnSoundatLocation "/Game/Sound/SoundEffect/Fuse2Sec.Fuse2Sec" (Transformation|GetActorLocation) "0, 0, 0" 1.0 1.0 0.0 0 0))
      (Variables|Default|SetFuzeRef _returnvalue)
      (bind _output_get_2 (Variables|Default|SetBarrelHealth (- (Variables|Default|GetBarrelHealth) 0.0)))
      (if (not (<= _output_get_2 0.0))
        (Utilities|FlowControl|Delay 2.0)
        (goto _label)))))

(fn ConstructionScript)