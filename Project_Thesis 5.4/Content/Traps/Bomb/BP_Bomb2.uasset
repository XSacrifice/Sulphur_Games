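; Hold-to-interact bomb trap that the player completes to add a bomb point toward passing the mission.
; Box overlap enables input, shows WB_Hold and opens a Gate; holding IA_Hold freezes movement while a self-calling event polls a timer for progress.
; After the hold delay it plays a shutter sound, increments BombPoint and hides the trap.
; Reaching MaxBombPoint swaps the timer widget for Mission Passed with an alarm; several unconnected leftover chains remain.
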(event OnComponentBeginOverlap(Box)
  (params (OverlappedComponent :type Primitive%20Component%20Object%20Reference) (OtherActor :type Actor%20Object%20Reference) (OtherComp :type Primitive%20Component%20Object%20Reference) (OtherBodyIndex :type Integer) (bFromSweep :type Boolean) (SweepResult :type Hit%20Result%20Structure%20%28by%20ref%29))
  (Utilities|Casting|CastToBP_Player OtherActor)
  (Input|EnableInput (Game|GetPlayerController 0))
  (bind _returnvalue (UserInterface|CreateWidget "/Game/ThirdPerson/UI/WB_Hold.WB_Hold_C"))
  (bind _output_get (Variables|Default|SetWidget%20REF _returnvalue))
  (UserInterface|Viewport|AddtoViewport _output_get 0)
  (Variables|/Game/ThirdPerson/UI/WB_Hold.WB_Hold_C|SetMaxTimeHeld _output_get (Variables|Default|GetMaxHoldTime))
  (Utilities|FlowControl|Gate true) ; enters at Open
)

(event OnComponentEndOverlap(Box)
  (params (OverlappedComponent :type Primitive%20Component%20Object%20Reference) (OtherActor :type Actor%20Object%20Reference) (OtherComp :type Primitive%20Component%20Object%20Reference) (OtherBodyIndex :type Integer))
  (Utilities|Casting|CastToBP_Player OtherActor)
  (Input|DisableInput (Game|GetPlayerController 0))
  (Widget|RemovefromParent (stale OnComponentBeginOverlap(Box) _returnvalue))
  (Utilities|FlowControl|Gate true) ; enters at Close
)

(event Custom|ColletBombPoint01
  (Math|Integer|IncrementInt (Variables|Default|GetBombPoint)
    (:%20%20
      (Development|PrintString "succeed")
      (Utilities|FlowControl|DoOnce false :!label _label
        (:Completed
          (if (== (Variables|Default|GetBombPoint) (Variables|Default|GetMaxBombPoint))
            (bind _foundwidgets (Widget|GetAllWidgetsOfClass "/Game/Map_Wall/WB_TimerGameWall.WB_TimerGameWall_C" true))
            (Widget|RemovefromParent _foundwidgets)
            (bind _returnvalue (UserInterface|CreateWidget "/Game/ThirdPerson/UI/MissionPassText/WB_MissionPassed.WB_MissionPassed_C"))
            (UserInterface|Viewport|AddtoViewport _returnvalue 0)
            (if true
              (Default|PlayMissionPassedAnimation _returnvalue)
              (Audio|PlaySound2D "/Game/Sound/SoundEffect/Alarm.Alarm" 1.0 1.0 0.0 0 0)
              (goto _label Reset))))))))

(event Custom|StopTimer
  (Utilities|Time|PauseTimerbyHandle (stale Custom|Timer _returnvalue)))

(event Custom|CollectItem
  (Math|Integer|IncrementInt (Variables|Default|Getfor%20bomb%20point)
    (:%20%20
      (Utilities|FlowControl|DoOnce false
        (:Completed
          (if true
            (CallFunction|ColletBombPoint01)))))))

(event Custom|UpdateTimer
  (bind _widget_ref (Variables|Default|GetWidget%20REF))
  (if (Variables|Default|GetIsHeld?)
    (Variables|/Game/ThirdPerson/UI/WB_Hold.WB_Hold_C|SetTimeHeld _widget_ref (Class|KismetSystemLibrary|GetTimerElapsedTimeHandle (stale Custom|Timer _returnvalue)))
    (Utilities|FlowControl|Delay 0.1)
    (CallFunction|UpdateTimer)
    (else
      (CallFunction|StopTimer)
      (Variables|/Game/ThirdPerson/UI/WB_Hold.WB_Hold_C|SetTimeHeld _widget_ref 0.0))))

(event Custom|Timer
  (bind _returnvalue (Utilities|Time|SetTimerbyEvent (delegate Custom|Timer) (Variables|Default|GetMaxHoldTime))))

(event Input|EnhancedActionEvents|EnhancedInputActionIA_Hold
  (params (ActionValue :type Boolean) (ElapsedSeconds :type Float%20%28double-precision%29) (TriggeredSeconds :type Float%20%28double-precision%29) (InputAction :type Input%20Action%20Object%20Reference :default "/Game/ThirdPerson/Input/Actions/IA_Hold.IA_Hold"))
  (:Triggered
    (Variables|Default|SetIsHeld? true)
    (Pawn|Components|CharacterMovement|SetMovementMode (Variables|/Script/Engine.Character|GetCharacterMovement (Game|GetPlayerCharacter 0)) "MOVE_None" 0)
    (Utilities|FlowControl|Gate true
      (:Exit
        (Utilities|FlowControl|Sequence
          (:then_0
            (Utilities|FlowControl|RetriggerableDelay (Variables|Default|GetMaxHoldTime))
            (Widget|RemovefromParent (stale OnComponentBeginOverlap(Box) _output_get))
            (if (Variables|Default|GetIsHeld?)
              (Audio|PlaySoundatLocation "/Engine/VREditor/Sounds/UI/Camera_Shutter.Camera_Shutter" "0, 0, 0" "0, 0, 0" 1.0 1.0 0.0 0 0 0 0)
              (Utilities|FlowControl|Delay 0.3)
              (CallFunction|CollectItem)
              (Utilities|FlowControl|Delay 0.1)
              (Development|SetHiddeninGame (Variables|Default|GetBox) true false)
              (Development|SetHiddeninGame (Variables|Default|GetPointLight) true false)
              (Development|SetHiddeninGame (Variables|Default|GetDynamiteTrap) true false)))
          (:then_1
            (CallFunction|Timer)
            (CallFunction|UpdateTimer))))))
  (:Completed
    (Variables|Default|SetIsHeld? false)
    (Pawn|Components|CharacterMovement|SetMovementMode (Variables|/Script/Engine.Character|GetCharacterMovement (Game|GetPlayerCharacter 0)) "MOVE_Walking" 0)))

(fn ConstructionScript)