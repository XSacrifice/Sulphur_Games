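; BP_InstantBomb is a tripwire-trap bomb that detonates on a short fuse as soon as it spawns.
; BeginPlay plays three warning beeps half a second apart, then applies radial damage around the actor.
; The blast also spawns a scaled-up explosion effect and sound and fires a RadialForce impulse before the actor destroys itself.
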(event EventBeginPlay
  (Audio|PlaySoundatLocation "/Game/Sound/SoundEffect/VendingMachine/VendingBeep.VendingBeep" (Transformation|GetActorLocation) "0, 0, 0" 1.0 1.0 0.0 0 0 0 0)
  (Utilities|FlowControl|Delay 0.5)
  (Audio|PlaySoundatLocation "/Game/Sound/SoundEffect/VendingMachine/VendingBeep.VendingBeep" (Transformation|GetActorLocation) "0, 0, 0" 1.0 1.0 0.0 0 0 0 0)
  (Utilities|FlowControl|Delay 0.5)
  (Audio|PlaySoundatLocation "/Game/Sound/SoundEffect/VendingMachine/VendingBeep.VendingBeep" (Transformation|GetActorLocation) "0, 0, 0" 1.0 1.0 0.0 0 0 0 0)
  (Utilities|FlowControl|Delay 0.5)
  (Game|Damage|ApplyRadialDamage 6e+01 (Transformation|GetActorLocation) 5e+02 0 0 self 0 false "ECC_Visibility")
  (Effects|SpawnEmitteratLocation "/Game/StarterContent/Particles/P_Explosion.P_Explosion" (Transformation|GetActorLocation) "0, 0, 0" "3.000000,3.000000,3.000000")
  (Audio|PlaySoundatLocation "/Game/Sound/SoundEffect/Audio/Explosion_Cue.Explosion_Cue" (Transformation|GetActorLocation) "0, 0, 0" 1.0 1.0 0.0 0 0 0 0)
  (Class|RadialForceComponent|FireImpulse (Variables|Default|GetRadialForce))
  (Actor|DestroyActor))

(fn ConstructionScript)