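; BP_AmmoPickuup is an ammo pickup that adds a fixed amount of ammo to the third-person player character on overlap.
; BeginPlay caches player 0's character, which each overlapping actor is compared against.
; A player overlap passes through a DoOnce, increments the character's Ammo and destroys the pickup.
; An overlap by any other actor destroys the pickup after a short delay without granting ammo.
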(event EventBeginPlay
  (bind _asbp_third_person_character (Utilities|Casting|CastToBP_ThirdPersonCharacter (Game|GetPlayerCharacter 0)))
  (Variables|Default|SetAs%20BP%20Third%20Person%20Character _asbp_third_person_character))

(event Collision|EventActorBeginOverlap
  (params (OtherActor :type Actor%20Object%20Reference))
  (bind _as_bp_third_person_character (Variables|Default|GetAs%20BP%20Third%20Person%20Character))
  (if (== OtherActor (Variables|Default|GetAs%20BP%20Third%20Person%20Character))
    (Utilities|FlowControl|DoOnce false
      (:Completed
        (Variables|/Game/ThirdPerson/Blueprints/Player/BP_ThirdPersonCharacter.BP_ThirdPersonCharacter_C|SetAmmo _as_bp_third_person_character (+ (Variables|/Game/ThirdPerson/Blueprints/Player/BP_ThirdPersonCharacter.BP_ThirdPersonCharacter_C|GetAmmo _as_bp_third_person_character) 10))
        (Actor|DestroyActor)))
    (else
      (Utilities|FlowControl|Delay 5.0)
      (Actor|DestroyActor))))

(event EventTick
  (params (DeltaSeconds :type Float%20%28single-precision%29)))

(fn ConstructionScript)