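; BP_TarGetSpawnPoint is a trigger, kept in the Unused folder, meant to start repeated target spawning.
; A Box overlap stores all actors tagged "Target" in TheTargetCreater and starts a looping timer for "TargetSpawn", a function not defined here.
; The interval uses modulo (1.0 % TargetSpawnEverySecond), while a division node sits unconnected.
; The overlapping actor is not checked; a Tps comparison is never run.
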(event OnComponentBeginOverlap(Box)
  (params (OverlappedComponent :type Primitive%20Component%20Object%20Reference) (OtherActor :type Actor%20Object%20Reference) (OtherComp :type Primitive%20Component%20Object%20Reference) (OtherBodyIndex :type Integer) (bFromSweep :type Boolean) (SweepResult :type Hit%20Result%20Structure%20%28by%20ref%29))
  (bind _outactors (Actor|GetAllActorswithTag "Target"))
  (bind _output_get (Variables|Default|SetTheTargetCreater _outactors))
  (Utilities|Time|SetTimerbyFunctionName 0 "TargetSpawn" (Math|Float|%(Float) 1.0 (Variables|Default|GetTargetSpawnEverySecond)) true))

(event EventBeginPlay)

(event Collision|EventActorBeginOverlap
  (params (OtherActor :type Actor%20Object%20Reference)))

(event EventTick
  (params (DeltaSeconds :type Float%20%28single-precision%29)))

(fn ConstructionScript)