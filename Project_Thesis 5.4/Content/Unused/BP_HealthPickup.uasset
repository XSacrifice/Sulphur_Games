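; BP_HealthPickup is a pickup actor that restores health to the player on overlapping its box.
; It caches the BP_Player character on BeginPlay, then through a DoOnce adds a fixed, clamped amount if health is below 1.0, updates health and destroys itself.
; The DoOnce precedes the health check and never resets, so a full-health touch uses up the heal.
; Overlaps by other actors destroy it after a delay, and Pickup destroys it immediately.
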(event OnComponentBeginOverlap(Box)
  (params (OverlappedComponent :type Primitive%20Component%20Object%20Reference) (OtherActor :type Actor%20Object%20Reference) (OtherComp :type Primitive%20Component%20Object%20Reference) (OtherBodyIndex :type Integer) (bFromSweep :type Boolean) (SweepResult :type Hit%20Result%20Structure%20%28by%20ref%29))
  (bind _as_bp_third_person_character (Variables|Default|GetAs%20BP%20Third%20Person%20Character))
  (if (== OtherActor (Variables|Default|GetAs%20BP%20Third%20Person%20Character))
    (Utilities|FlowControl|DoOnce false
      (:Completed
        (if (< (Variables|/Game/Characters_Added/Player/BP_Player.BP_Player_C|GetHealth (Variables|Default|GetAs%20BP%20Third%20Person%20Character)) 1.0)
          (Variables|/Game/Characters_Added/Player/BP_Player.BP_Player_C|SetHealth _as_bp_third_person_character (Math|Float|Clamp(Float) (+ (Variables|/Game/Characters_Added/Player/BP_Player.BP_Player_C|GetHealth _as_bp_third_person_character) 0.5) 0.0 (Variables|/Game/Characters_Added/Player/BP_Player.BP_Player_C|GetMaxHealth _as_bp_third_person_character)))
          (Default|UpdateHealth (Variables|Default|GetAs%20BP%20Third%20Person%20Character))
          (Actor|DestroyActor))))
    (else
      (Utilities|FlowControl|Delay 5.0)
      (Actor|DestroyActor))))

(event EventBeginPlay
  (bind _asbp_third_person_character (Utilities|Casting|CastToBP_Player (Game|GetPlayerCharacter 0)))
  (Variables|Default|SetAs%20BP%20Third%20Person%20Character _asbp_third_person_character))

(event EventPickup
  (params (CharacterPickUp :type BP%20Player%20Object%20Reference))
  (Actor|DestroyActor))

(event Input|KeyboardEvents|E
  (params (Key :type Key%20Structure)))

(fn ConstructionScript)