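; Trigger actor that, judging by its name and calls, is meant to clear the objective widget when its box is overlapped.
; The first box overlap calls CloseWB, which is guarded by a counter and DoOnce nodes to run only once.
; CloseWB creates a new WB_Objective, immediately calls RemoveFromParent on that new instance rather than an existing one, then destroys the actor.
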(event OnComponentBeginOverlap(Box)
  (params (OverlappedComponent :type Primitive%20Component%20Object%20Reference) (OtherActor :type Actor%20Object%20Reference) (OtherComp :type Primitive%20Component%20Object%20Reference) (OtherBodyIndex :type Integer) (bFromSweep :type Boolean) (SweepResult :type Hit%20Result%20Structure%20%28by%20ref%29))
  (Utilities|FlowControl|DoOnce false
    (:Completed
      (Utilities|FlowControl|Sequence
        (:then_0
          (CallFunction|CloseWB))))))

(event Custom|CloseWB
  (Math|Integer|IncrementInt (Variables|Default|Getclose)
    (:%20%20
      (if (== (Variables|Default|Getclose) 1)
        (Utilities|FlowControl|DoOnce false
          (:Completed
            (bind _returnvalue (UserInterface|CreateWidget "/Game/Characters/Player/Blueprint/Widget/WB_Objective.WB_Objective_C"))
            (if true
              (Widget|RemovefromParent _returnvalue)
              (Actor|DestroyActor))))))))

(event Collision|EventActorBeginOverlap
  (params (OtherActor :type Actor%20Object%20Reference)))

(fn ConstructionScript)