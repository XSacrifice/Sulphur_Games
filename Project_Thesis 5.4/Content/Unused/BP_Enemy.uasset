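; Enemy pawn that chases the player, deals contact damage and drops loot on death.
; PawnSensing sets a seen flag, never cleared here, and issues an AI MoveTo toward the player character.
; Capsule overlap applies small random damage to any overlapping actor, while incoming damage drains health until the enemy destroys itself.
; On death it runs random loot rolls, tracing downward to place health or pistol ammo pickups with random yaw.
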(event OnSeePawn(PawnSensing)
  (params (Pawn :type Pawn%20Object%20Reference))
  (Variables|Default|SetisSeeingPlayer? true)
  (CallFunction|FollowPlayer))

(event OnComponentBeginOverlap(Capsule)
  (params (OverlappedComponent :type Primitive%20Component%20Object%20Reference) (OtherActor :type Actor%20Object%20Reference) (OtherComp :type Primitive%20Component%20Object%20Reference) (OtherBodyIndex :type Integer) (bFromSweep :type Boolean) (SweepResult :type Hit%20Result%20Structure%20%28by%20ref%29))
  (Game|Damage|ApplyDamage OtherActor (Math|Random|RandomFloatinRange 0.02 0.05) 0 self))

(event Custom|DropLoot
  (bind _returnvalue (Transformation|GetActorLocation))
  (bind _outhit (Collision|LineTraceByChannel _returnvalue (- _returnvalue "0.000000,0.000000,200.000000") "TraceTypeQuery1" false (Utilities|Array|MakeArray (Game|GetPlayerCharacter 0)) "None"))
  (Game|SpawnActorfromClass (Utilities|Select :Index (Math|Random|RandomInteger 3) :Option%200 "/Game/Unused/BP_HealthPickup.BP_HealthPickup_C" :Option%201 "/Game/ThirdPerson/Blueprints/Item/BP_PistolAmmoPickuup1.BP_PistolAmmoPickuup1_C" :Option%202 0 :Option%203 0) (Math|Transform|MakeTransform (.Location (Collision|BreakHitResult _outhit)) (Math|Rotator|MakeRotator 0.0 0.0 (Math|Random|RandomFloatinRange 0.0 3.6e+02))) "AlwaysSpawn" "MultiplyWithRoot" 0 0))

(event Custom|FollowPlayer
  (if (Variables|Default|GetisSeeingPlayer?)
    (AI|AIMoveTo self "0, 0, 0" (Game|GetPlayerCharacter 0) 5.0 false)))

(event EventBeginPlay)

(event Collision|EventActorBeginOverlap
  (params (OtherActor :type Actor%20Object%20Reference)))

(event EventTick
  (params (DeltaSeconds :type Float%20%28single-precision%29)))

(event Game|Damage|EventAnyDamage
  (params (Damage :type Float%20%28single-precision%29) (DamageType :type Damage%20Type%20Object%20Reference) (InstigatedBy :type Controller%20Object%20Reference) (DamageCauser :type Actor%20Object%20Reference))
  (bind _output_get (Variables|Default|SetEnemyHealth (- (Variables|Default|GetEnemyHealth) Damage)))
  (if (<= _output_get 0.0)
    (for _index (range 0 (Math|Random|RandomInteger 3))
      (CallFunction|DropLoot))
    (Actor|DestroyActor)))

(fn ConstructionScript)