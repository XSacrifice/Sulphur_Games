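; BP_AImoveto1 is an enemy, stored in an Unused folder, that chases the player and can be killed by damage.
; On BeginPlay it casts player character 0 to BP_Player and issues a single AI MoveTo toward it.
; AnyDamage subtracts from EnemyHealth and destroys the actor at zero or below.
; Sight-based following through IsSeeingPlayer and FollowPlayer is present but never executes.
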(event EventBeginPlay
  (bind _asbp_third_person_character (Utilities|Casting|CastToBP_Player (Game|GetPlayerCharacter 0)))
  (AI|AIMoveTo 0 "0, 0, 0" _asbp_third_person_character 5.0 false))

(event Collision|EventActorBeginOverlap
  (params (OtherActor :type Actor%20Object%20Reference)))

(event EventTick
  (params (DeltaSeconds :type Float%20%28single-precision%29)))

(event Game|Damage|EventAnyDamage
  (params (Damage :type Float%20%28single-precision%29) (DamageType :type Damage%20Type%20Object%20Reference) (InstigatedBy :type Controller%20Object%20Reference) (DamageCauser :type Actor%20Object%20Reference))
  (bind _output_get (Variables|Default|SetEnemyHealth (- (Variables|Default|GetEnemyHealth) Damage)))
  (if (<= _output_get 0.0)
    (Actor|DestroyActor)))

(fn ConstructionScript)