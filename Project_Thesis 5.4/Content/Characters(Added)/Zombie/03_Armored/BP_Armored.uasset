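; BP_Armored is an armored zombie enemy that takes damage, attacks the player and drops loot on death.
; AnyDamage reduces health, playing a hit sound or spawning random health or pistol-ammo pickups at a downward trace before destroying itself.
; Attack plays a montage and debug feedback, then damages the cached player after a delay without a range check.
; Chase and EQS logic is disconnected, so nothing here triggers Attack.
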(event Custom|FollowPlayer)

(event Custom|DropLoot
  (bind _returnvalue (Transformation|GetActorLocation))
  (bind _outhit (Collision|LineTraceByChannel _returnvalue (- _returnvalue "0.000000,0.000000,200.000000") "TraceTypeQuery1" false (Utilities|Array|MakeArray (Game|GetPlayerCharacter 0)) "None"))
  (Game|SpawnActorfromClass (Utilities|Select :Index (Math|Random|RandomInteger 8) :Option%200 "/Game/ThirdPerson/Blueprints/Item/BP_HealthPickup2_PickToUse.BP_HealthPickup2_PickToUse_C" :Option%201 0 :Option%202 "/Game/ThirdPerson/Blueprints/Item/BP_PistolAmmoPickuup_8.BP_PistolAmmoPickuup_8_C" :Option%203 "/Game/ThirdPerson/Blueprints/Item/BP_PistolAmmoPickuup_3.BP_PistolAmmoPickuup_3_C" :Option%204 "/Game/ThirdPerson/Blueprints/Item/BP_PistolAmmoPickuup_1.BP_PistolAmmoPickuup_1_C" :Option%205 "/Game/ThirdPerson/Blueprints/Item/BP_PistolAmmoPickuup_1.BP_PistolAmmoPickuup_1_C" :Option%206 0 :Option%207 0 :Option%208 0) (Math|Transform|MakeTransform (.Location (Collision|BreakHitResult _outhit)) (Math|Rotator|MakeRotator 0.0 0.0 (Math|Random|RandomFloatinRange 0.0 3.6e+02))) "AlwaysSpawn" "MultiplyWithRoot" 0 0))

(event Custom|Attack
  (Animation|PlayAnimMontage "/Game/Characters(Added)/Zombie/01_Walker/Animation/anim_zombie_a_attack_Montage.anim_zombie_a_attack_Montage" 1.0 "None")
  (Utilities|FlowControl|Sequence
    (:then_0
      (Audio|PlaySound2D "/Engine/EngineSounds/1kSineTonePing.1kSineTonePing" 1.0 1.0 0.0 0 0)
      (Development|PrintString "Hit"))
    (:then_1
      (Utilities|FlowControl|Delay 1.0)
      (Game|Damage|ApplyDamage (Variables|Default|GetAs%20BP%20Third%20Person%20Character) 0.1 0 (Variables|Default|GetAs%20BP%20Third%20Person%20Character)))))

(event EventBeginPlay
  (bind _asbp_third_person_character (Utilities|Casting|CastToBP_ThirdPersonCharacter (Game|GetPlayerCharacter 0)))
  (Variables|Default|SetAs%20BP%20Third%20Person%20Character _asbp_third_person_character)
  (if (== (Variables|Default|GetEnemyHealth) 0.0)
    (Actor|DestroyActor)))

(event Collision|EventActorBeginOverlap
  (params (OtherActor :type Actor%20Object%20Reference)))

(event EventTick
  (params (DeltaSeconds :type Float%20%28single-precision%29)))

(event Game|Damage|EventAnyDamage
  (params (Damage :type Float%20%28single-precision%29) (DamageType :type Damage%20Type%20Object%20Reference) (InstigatedBy :type Controller%20Object%20Reference) (DamageCauser :type Actor%20Object%20Reference))
  (bind _output_get (Variables|Default|SetEnemyHealth (- (Variables|Default|GetEnemyHealth) Damage)))
  (if (<= _output_get 0.0)
    (for _index (range 0 (Math|Random|RandomInteger 2))
      (CallFunction|DropLoot))
    (Actor|DestroyActor)
    (else
      (Audio|PlaySoundatLocation "/Game/SoundEffect/DrumHIt.DrumHIt" (Transformation|GetActorLocation) "0, 0, 0" 1.0 1.0 0.0 0 0 0 0))))

(fn ConstructionScript)