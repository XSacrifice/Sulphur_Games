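; BP_ScrapMachine is a shop machine that refines the player's currency into a BP_BScrap pickup actor.
; The overlap box shows a press-E widget, enables input and opens a Gate for the key.
; Pressing E spends currency if affordable and the machine is idle, then runs a timed refining cycle before spawning the scrap at the Arrow.
; Stored audio references switch the waiting and refining sounds, though waiting audio starts only at BeginPlay.
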(event OnComponentBeginOverlap(Box)
  (params (OverlappedComponent :type Primitive%20Component%20Object%20Reference) (OtherActor :type Actor%20Object%20Reference) (OtherComp :type Primitive%20Component%20Object%20Reference) (OtherBodyIndex :type Integer) (bFromSweep :type Boolean) (SweepResult :type Hit%20Result%20Structure%20%28by%20ref%29))
  (bind _arrow (Variables|Default|GetArrow))
  (bind _returnvalue (Transformation|GetWorldLocation _arrow))
  (Utilities|Casting|CastToBP_Player OtherActor)
  (Input|EnableInput (Game|GetPlayerController 0))
  (bind _returnvalue_2 (UserInterface|CreateWidget "/Game/ThirdPerson/UI/WB_PressE.WB_PressE_C"))
  (bind _output_get (Variables|Default|SetPress%20E%20Ref _returnvalue_2))
  (UserInterface|Viewport|AddtoViewport _output_get 0)
  (Utilities|FlowControl|Gate true) ; enters at Open
)

(event OnComponentEndOverlap(Box)
  (params (OverlappedComponent :type Primitive%20Component%20Object%20Reference) (OtherActor :type Actor%20Object%20Reference) (OtherComp :type Primitive%20Component%20Object%20Reference) (OtherBodyIndex :type Integer))
  (bind _arrow (Variables|Default|GetArrow))
  (bind _returnvalue (Transformation|GetWorldLocation _arrow))
  (Utilities|Casting|CastToBP_Player OtherActor)
  (Input|DisableInput (Game|GetPlayerController 0))
  (Widget|RemovefromParent (stale OnComponentBeginOverlap(Box) _returnvalue_2))
  (Utilities|FlowControl|Gate true) ; enters at Close
)

(event Collision|EventActorBeginOverlap
  (params (OtherActor :type Actor%20Object%20Reference)))

(event EventTick
  (params (DeltaSeconds :type Float%20%28single-precision%29)))

(event EventBeginPlay
  (if (not (Variables|Default|GetRefining?))
    (bind _returnvalue (Audio|SpawnSoundatLocation "/Game/Sound/SoundEffect/CoinMachine/CoinMachineWating.CoinMachineWating" (Transformation|GetActorLocation) "0, 0, 0" 1.0 1.0 0.0 0 0))
    (Variables|Default|SetWaitingCoinRef _returnvalue)))

(event Input|KeyboardEvents|E
  (params (Key :type Key%20Structure :default "None"))
  (bind _arrow (Variables|Default|GetArrow))
  (bind _returnvalue (Transformation|GetWorldLocation _arrow))
  (:Pressed
    (Utilities|FlowControl|Gate true
      (:Exit
        (Utilities|FlowControl|Sequence
          (:then_0
            (bind _asbp_player (Utilities|Casting|CastToBP_Player (Game|GetPlayerCharacter 0)))
            (if (>= (Variables|/Game/Characters_Added/Player/BP_Player.BP_Player_C|GetCurrency _asbp_player) 4)
              (if (Variables|Default|GetRefining?)
                (Development|PrintString "refining")
                (else
                  (Default|ReduceCurrency _asbp_player 4)
                  (Variables|Default|SetRefining? true)
                  (if (Variables|Default|GetRefining?)
                    (Audio|Components|Audio|Stop (Variables|Default|GetWaitingCoinRef))
                    (Audio|PlaySoundatLocation "/Game/Sound/SoundEffect/Audio/Selected.Selected" (Transformation|GetActorLocation) "0, 0, 0" 1.0 1.0 0.0 0 0 0 0)
                    (Utilities|FlowControl|Delay 1.0)
                    (bind _returnvalue_2 (Audio|SpawnSoundatLocation "/Game/Sound/SoundEffect/CoinMachine/CoinMachineRefining.CoinMachineRefining" (Transformation|GetActorLocation) "0, 0, 0" 1.0 1.0 0.0 0 0))
                    (Variables|Default|SetReSongRef _returnvalue_2)
                    (Utilities|FlowControl|Delay 3e+01)
                    (Variables|Default|SetRefining? false)
                    (Game|SpawnActorfromClass "/Game/Shop/BP_BScrap.BP_BScrap_C" (Math|Conversions|ToTransform(Vector) (Transformation|GetWorldLocation (Variables|Default|GetArrow))) "Undefined" "MultiplyWithRoot" 0 0)
                    (Audio|PlaySoundatLocation "/Engine/EngineSounds/1kSineTonePing.1kSineTonePing" _returnvalue "0, 0, 0" 1.0 1.0 0.0 0 0 0 0)
                    (Audio|PlaySoundatLocation "/Game/Sound/SoundEffect/CoinDrop.CoinDrop" _returnvalue "0, 0, 0" 1.0 1.0 0.0 0 0 0 0)
                    (Audio|Components|Audio|Stop (Variables|Default|GetReSongRef)))))
              (else
                (Development|PrintString "No Scrap")))))))))

(fn ConstructionScript)