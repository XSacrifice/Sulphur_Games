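; BP_SScrap is a scrap pickup that gives the player one currency, plays a coin sound and destroys itself.
; Collection happens either through the Pickup event or automatically when BP_Player overlaps the Box component.
; A separate InteractBox shows a widget and applies an outline overlay material to the Cube while the player is inside, clearing both on exit.
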(event OnComponentBeginOverlap(Box)
  (params (OverlappedComponent :type Primitive%20Component%20Object%20Reference) (OtherActor :type Actor%20Object%20Reference) (OtherComp :type Primitive%20Component%20Object%20Reference) (OtherBodyIndex :type Integer) (bFromSweep :type Boolean) (SweepResult :type Hit%20Result%20Structure%20%28by%20ref%29))
  (bind _asbp_player (Utilities|Casting|CastToBP_Player OtherActor))
  (Default|AddCurrency _asbp_player 1)
  (Audio|PlaySound2D "/Game/Sound/SoundEffect/CoinCue.CoinCue" 1.0 1.0 0.0 0 0)
  (Actor|DestroyActor))

(event OnComponentBeginOverlap(InteractBox)
  (params (OverlappedComponent :type Primitive%20Component%20Object%20Reference) (OtherActor :type Actor%20Object%20Reference) (OtherComp :type Primitive%20Component%20Object%20Reference) (OtherBodyIndex :type Integer) (bFromSweep :type Boolean) (SweepResult :type Hit%20Result%20Structure%20%28by%20ref%29))
  (if (== OtherActor (Variables|Default|GetAs%20BP%20Player))
    (Rendering|SetVisibility (Variables|Default|GetWidget) true false)
    (Rendering|Material|SetOverlayMaterial (Variables|Default|GetCube) "/Game/Props/00_Material/01_Special_Material/M_Outline/M_Outline_Inst.M_Outline_Inst" :!class /Script/Engine.MeshComponent)))

(event OnComponentEndOverlap(InteractBox)
  (params (OverlappedComponent :type Primitive%20Component%20Object%20Reference) (OtherActor :type Actor%20Object%20Reference) (OtherComp :type Primitive%20Component%20Object%20Reference) (OtherBodyIndex :type Integer))
  (if (== OtherActor (Variables|Default|GetAs%20BP%20Player))
    (Rendering|SetVisibility (Variables|Default|GetWidget) false false)
    (Rendering|Material|SetOverlayMaterial (Variables|Default|GetCube) 0 :!class /Script/Engine.MeshComponent)))

(event EventBeginPlay
  (bind _asbp_player (Utilities|Casting|CastToBP_Player (Game|Player|GetPlayerPawn 0)))
  (Variables|Default|SetAs%20BP%20Player _asbp_player))

(event Collision|EventActorBeginOverlap
  (params (OtherActor :type Actor%20Object%20Reference)))

(event EventTick
  (params (DeltaSeconds :type Float%20%28single-precision%29)))

(event EventPickup
  (params (CharacterPickUp :type BP%20Player%20Object%20Reference))
  (bind _asbp_player (Utilities|Casting|CastToBP_Player (Game|GetPlayerCharacter 0)))
  (Default|AddCurrency _asbp_player 1)
  (Audio|PlaySound2D "/Game/Sound/SoundEffect/CoinCue.CoinCue" 1.0 1.0 0.0 0 0)
  (Actor|DestroyActor))

(fn ConstructionScript)