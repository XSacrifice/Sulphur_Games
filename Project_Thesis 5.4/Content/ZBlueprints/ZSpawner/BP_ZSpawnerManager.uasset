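; Zombie spawner manager that triggers spawn points on timed intervals during play.
; Tick accumulates delta time into a whole-second counter, and once it passes a start threshold, each interval in an array is checked by modulo.
; A matching interval sends a spawn message to the spawn location at the same index and increments a round counter, whose reset and length check are left unconnected.
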(event Custom|Timer
  ;[1 1 1] Timer
  (bind _output_get (Variables|Default|Settime (+ (Variables|Default|Gettime) (Utilities|Time|GetWorldDeltaSeconds))))
  ;[1 1 1] Counter Sec
  (if (== (Math|Float|Truncate _output_get) (Variables|Default|Getseccount))
    (Variables|Default|Setseccount (+ (Variables|Default|Getseccount) 1))
    ;[1 1 1] Spawn Start Condition
    (if (>= (Variables|Default|Getseccount) (Variables|Default|Getstart_at))
      ;[1 1 1] Get Spawn Target Sec Time
      (for (_array_element _array_index) (Variables|Default|Getspawn_every_sec)
        (if (== (Math|Integer|%(Integer) (Variables|Default|Getseccount) _array_element) 0)
          (Class|BPZSpawnComm|ZSpawnComm(Message) (Utilities|Array|Get(acopy) (Variables|Default|Getspawn_location) _array_index))
          ;[1 1 1] Location Round Controller
          (Math|Integer|IncrementInt (Variables|Default|Getround)))))))

(event EventTick
  (params (DeltaSeconds :type Float%20%28single-precision%29))
  ;[1 1 1] In Game
  (CallFunction|Timer))

(fn ConstructionScript)