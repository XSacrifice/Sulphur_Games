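; BP_Walker is the basic walker zombie enemy, with melee attacks, damage reactions, death and scrap drops.
; A sphere overlap gates attacks fired through checkplayer; random montages open a short hit window in which hand-box overlaps damage the player.
; Lethal damage ragdolls it away from the damage causer, randomly drops scrap, with a possible skill-card bonus, then destroys it after a delay.
; Movement and AI chase nodes here are disconnected.
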(event OnComponentBeginOverlap(Sphere)
  (params (OverlappedComponent :type Primitive%20Component%20Object%20Reference) (OtherActor :type Actor%20Object%20Reference) (OtherComp :type Primitive%20Component%20Object%20Reference) (OtherBodyIndex :type Integer) (bFromSweep :type Boolean) (SweepResult :type Hit%20Result%20Structure%20%28by%20ref%29))
  (Utilities|Casting|CastToBP_Player OtherActor)
  (Variables|Default|SetZombie%20can%20Attack? true))

(event OnComponentEndOverlap(Sphere)
  (params (OverlappedComponent :type Primitive%20Component%20Object%20Reference) (OtherActor :type Actor%20Object%20Reference) (OtherComp :type Primitive%20Component%20Object%20Reference) (OtherBodyIndex :type Integer))
  (Utilities|Casting|CastToBP_Player OtherActor)
  (Variables|Default|SetZombie%20can%20Attack? false))

(event OnComponentBeginOverlap(BoxR)
  (params (OverlappedComponent :type Primitive%20Component%20Object%20Reference) (OtherActor :type Actor%20Object%20Reference) (OtherComp :type Primitive%20Component%20Object%20Reference) (OtherBodyIndex :type Integer) (bFromSweep :type Boolean) (SweepResult :type Hit%20Result%20Structure%20%28by%20ref%29))
  (Utilities|Casting|CastToBP_Player OtherActor)
  (Utilities|FlowControl|DoOnce false :!label _label
    (:Completed
      (if (Variables|Default|GetHit?)
        (Variables|Default|SethandR true)
        (CallFunction|Hit)
        (Utilities|FlowControl|Delay 1.0)
        (Variables|Default|SethandR false)
        (goto _label Reset)))))

(event OnComponentBeginOverlap(Box)
  (params (OverlappedComponent :type Primitive%20Component%20Object%20Reference) (OtherActor :type Actor%20Object%20Reference) (OtherComp :type Primitive%20Component%20Object%20Reference) (OtherBodyIndex :type Integer) (bFromSweep :type Boolean) (SweepResult :type Hit%20Result%20Structure%20%28by%20ref%29))
  (Utilities|Casting|CastToBP_Player OtherActor)
  (Utilities|FlowControl|DoOnce false :!label _label
    (:Completed
      (if (Variables|Default|GetHit?)
        (Variables|Default|SethandL true)
        (CallFunction|Hit)
        (Utilities|FlowControl|Delay 1.0)
        (Variables|Default|SethandL false)
        (goto _label Reset)))))

(event Custom|FollowPlayer)

(event Custom|Droploot%20SkillCard
  (bind _returnvalue (Transformation|GetActorLocation))
  (Variables|Default|SetIs%20Dropped? true)
  (Game|SpawnActorfromClass "/Game/Shop/BP_SScrap.BP_SScrap_C" (Math|Conversions|ToTransform(Vector) (- _returnvalue "0.000000,0.000000,100.000000")) "AlwaysSpawn" "MultiplyWithRoot" 0 0)
  (bind _outhit (Collision|LineTraceByChannel _returnvalue (- _returnvalue "0.000000,0.000000,200.000000") "TraceTypeQuery1" false (Utilities|Array|MakeArray (Game|GetPlayerCharacter 0)) "None"))
  (Game|SpawnActorfromClass (Utilities|Select :Index (Math|Random|RandomInteger 5) :Option%200 "/Game/Shop/BP_SScrap.BP_SScrap_C" :Option%201 0 :Option%202 0 :Option%203 0 :Option%204 0) (Math|Transform|MakeTransform (.Location (Collision|BreakHitResult _outhit)) (Math|Rotator|MakeRotator 0.0 0.0 (Math|Random|RandomFloatinRange 0.0 3.6e+02))) "AlwaysSpawn" "MultiplyWithRoot" 0 0))

(event Custom|Attack
  (if (not (Variables|Default|GetIsDead))
    (Utilities|FlowControl|DoOnce false :!label _label
      (:Completed
        (Animation|PlayAnimMontage (.OutItem (Utilities|Array|Random (Utilities|Array|MakeArray (Variables|Default|GetAttack%20Animation%20Montage_1) (Variables|Default|GetAttack%20Animation%20Montage_2)))) 1.0 "None")
        (Variables|Default|SetHit? true)
        (Utilities|FlowControl|Delay 0.5)
        (Audio|PlaySoundatLocation "/Game/Sound/Human/Cue/ZBite.ZBite" (Transformation|GetActorLocation) "0, 0, 0" 1.0 1.0 0.0 0 0 0 0)
        (Variables|Default|SetHit? false)
        (goto _label Reset)))))

(event Custom|Hit
  (if (not (Variables|Default|GetIsDead))
    (if (Variables|Default|GetHit?)
      (Utilities|FlowControl|Sequence
        (:then_0
          (if (Variables|Default|GethandR)
            (Game|Damage|ApplyDamage (Variables|Default|GetAs%20BP%20Third%20Person%20Character) 1e+01 0 self :!label _label)
            (Default|PlayerGotDamage (Variables|Default|GetAs%20BP%20Third%20Person%20Character))))
        (:then_1
          (if (Variables|Default|GethandL)
            (goto _label)))))))

(event Custom|DropLoot
  (bind _returnvalue (Transformation|GetActorLocation))
  (Variables|Default|SetIs%20Dropped? true)
  (Game|SpawnActorfromClass "/Game/Shop/BP_SScrap.BP_SScrap_C" (Math|Conversions|ToTransform(Vector) (- _returnvalue "0.000000,0.000000,100.000000")) "AlwaysSpawn" "MultiplyWithRoot" 0 0)
  (bind _outhit (Collision|LineTraceByChannel _returnvalue (- _returnvalue "0.000000,0.000000,200.000000") "TraceTypeQuery1" false (Utilities|Array|MakeArray (Game|GetPlayerCharacter 0)) "None"))
  (Game|SpawnActorfromClass (Utilities|Select :Index (Math|Random|RandomInteger 12) :Option%200 "/Game/Shop/BP_MScrap.BP_MScrap_C" :Option%201 0 :Option%202 0 :Option%203 0 :Option%204 0 :Option%205 0 :Option%206 0 :Option%207 0 :Option%208 0 :Option%209 0 :Option%2010 0 :Option%2011 0 :Option%2012 0) (Math|Transform|MakeTransform (.Location (Collision|BreakHitResult _outhit)) (Math|Rotator|MakeRotator 0.0 0.0 (Math|Random|RandomFloatinRange 0.0 3.6e+02))) "AlwaysSpawn" "MultiplyWithRoot" 0 0))

(event Custom|AnyPush)

(event Custom|check%20player
  (if (Variables|Default|GetZombie%20can%20Attack?)
    (CallFunction|Attack)))

(event EventBeginPlay
  (bind _asbp_player (Utilities|Casting|CastToBP_Player (Game|GetPlayerCharacter 0)))
  (Variables|Default|SetAs%20BP%20Third%20Person%20Character _asbp_player))

(event Collision|EventActorBeginOverlap
  (params (OtherActor :type Actor%20Object%20Reference)))

(event EventTick
  (params (DeltaSeconds :type Float%20%28single-precision%29)))

(event Game|Damage|EventAnyDamage
  (params (Damage :type Float%20%28single-precision%29) (DamageType :type Damage%20Type%20Object%20Reference) (InstigatedBy :type Controller%20Object%20Reference) (DamageCauser :type Actor%20Object%20Reference))
  (bind _mesh (Variables|Character|GetMesh))
  ;[1 1 1] Dead
  (Audio|PlaySoundatLocation "/Game/MilitaryWeapDark/Sound/Shotgun/Shotgun_ImpactBody_Cue.Shotgun_ImpactBody_Cue" (Transformation|GetActorLocation) "0, 0, 0" 1.0 1.0 0.0 0 0 0 0)
  (Variables|Default|SetDamage%20Causer DamageCauser)
  (bind _output_get (Variables|Default|SetWalker_CurrentHealth (- (Variables|Default|GetWalker_CurrentHealth) Damage)))
  (if (<= _output_get 0.0)
    (if (Variables|Default|GetIsDead)
      (Variables|Default|SetIs%20Dropped? true)
      (else
        (Audio|PlaySoundatLocation "/Game/Sound/Human/BigZombieDeath.BigZombieDeath" (Transformation|GetActorLocation) "0, 0, 0" 1.0 1.0 0.0 0 0 0 0)))
    (for _index (range 0 (Math|Random|RandomInteger 2))
      (if (not (Variables|Default|GetIsDead))
        (if (not (Variables|Default|GetIs%20Dropped?))
          (bind _asbp_player (Utilities|Casting|CastToBP_Player (Game|GetPlayerCharacter 0)))
          (CallFunction|DropLoot)
          (if (Variables|/Game/Characters_Added/Player/BP_Player.BP_Player_C|GetGot%20shot? _asbp_player)
            (if (Variables|/Game/Characters_Added/Player/BP_Player.BP_Player_C|GetSkill%20Card50%25%20MoneyWhenGotShot _asbp_player)
              (CallFunction|DroplootSkillCard))))))
    (Pawn|Components|CharacterMovement|DisableMovement (Variables|Character|GetCharacterMovement))
    (Variables|Default|SetIsDead true)
    (Physics|SetSimulatePhysics _mesh true)
    (Physics|AddImpulse _mesh (* (Math|Vector|Normalize (- (Transformation|GetActorLocation) (Transformation|GetActorLocation (Variables|Default|GetDamage%20Causer)))) 500) "None" true)
    (Collision|SetCollisionResponsetoChannel (Variables|Character|GetMesh) "ECC_Visibility" "ECR_Ignore")
    (Collision|SetCollisionResponsetoChannel (Variables|Character|GetMesh) "ECC_Pawn" "ECR_Ignore")
    (Utilities|FlowControl|Delay 8.0)
    (Actor|DestroyActor)
    (elif (not (Variables|Default|GetIsDead))
      (Audio|PlaySoundatLocation "/Game/Sound/Human/BigZGrunt.BigZGrunt" (Transformation|GetActorLocation) "0, 0, 0" 1.0 1.0 0.0 0 0 0 0))))

(fn ConstructionScript)