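; BP_TrapBomb is a tripwire bomb trap that explodes on contact or when its health runs out.
; Box overlap casts for the player or four enemy types, then applies radial damage, sound and a force impulse, with weaker damage for player triggers.
; Depleted TripwireHealth triggers a randomly repeated blast that also calls PlayerGotDamage.
; Incoming radial damage destroys it with only an explosion effect; enemy-triggered overlaps spawn no emitter themselves.
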(event OnComponentBeginOverlap(Box)
  (params (OverlappedComponent :type Primitive%20Component%20Object%20Reference) (OtherActor :type Actor%20Object%20Reference) (OtherComp :type Primitive%20Component%20Object%20Reference) (OtherBodyIndex :type Integer) (bFromSweep :type Boolean) (SweepResult :type Hit%20Result%20Structure%20%28by%20ref%29))
  (Utilities|FlowControl|Sequence
    (:then_0
      (Utilities|Casting|CastToBP_Player OtherActor)
      (Game|Damage|ApplyRadialDamage 6e+01 (Transformation|GetActorLocation) 5e+02 0 0 self 0 false "ECC_Visibility")
      (Effects|SpawnEmitteratLocation "/Game/StarterContent/Particles/P_Explosion.P_Explosion" (Transformation|GetActorLocation) "0, 0, 0" "3.000000,3.000000,3.000000")
      (Audio|PlaySoundatLocation "/Game/Sound/SoundEffect/Audio/Explosion_Cue.Explosion_Cue" (Transformation|GetActorLocation) "0, 0, 0" 1.0 1.0 0.0 0 0 0 0)
      (Class|RadialForceComponent|FireImpulse (Variables|Default|GetRadialForce))
      (Actor|DestroyActor))
    (:then_1
      (Utilities|Casting|CastToBP_Walker OtherActor)
      (Game|Damage|ApplyRadialDamage 1e+02 (Transformation|GetActorLocation) 5e+02 0 0 self 0 false "ECC_Visibility")
      (Audio|PlaySoundatLocation "/Game/Sound/SoundEffect/Audio/Explosion_Cue.Explosion_Cue" (Transformation|GetActorLocation) "0, 0, 0" 1.0 1.0 0.0 0 0 0 0)
      (Class|RadialForceComponent|FireImpulse (Variables|Default|GetRadialForce))
      (Actor|DestroyActor))
    (:then_2
      (Utilities|Casting|CastToBP_Freak OtherActor)
      (Game|Damage|ApplyRadialDamage 1e+02 (Transformation|GetActorLocation) 5e+02 0 0 self 0 false "ECC_Visibility")
      (Audio|PlaySoundatLocation "/Game/Sound/SoundEffect/Audio/Explosion_Cue.Explosion_Cue" (Transformation|GetActorLocation) "0, 0, 0" 1.0 1.0 0.0 0 0 0 0)
      (Class|RadialForceComponent|FireImpulse (Variables|Default|GetRadialForce))
      (Actor|DestroyActor))
    (:then_3
      (Utilities|Casting|CastToBP_Sprinter OtherActor)
      (Game|Damage|ApplyRadialDamage 1e+02 (Transformation|GetActorLocation) 5e+02 0 0 self 0 false "ECC_Visibility")
      (Audio|PlaySoundatLocation "/Game/Sound/SoundEffect/Audio/Explosion_Cue.Explosion_Cue" (Transformation|GetActorLocation) "0, 0, 0" 1.0 1.0 0.0 0 0 0 0)
      (Class|RadialForceComponent|FireImpulse (Variables|Default|GetRadialForce))
      (Actor|DestroyActor))
    (:then_4
      (Utilities|Casting|CastToBP_Armored OtherActor)
      (Game|Damage|ApplyRadialDamage 1e+02 (Transformation|GetActorLocation) 5e+02 0 0 self 0 false "ECC_Visibility")
      (Audio|PlaySoundatLocation "/Game/Sound/SoundEffect/Audio/Explosion_Cue.Explosion_Cue" (Transformation|GetActorLocation) "0, 0, 0" 1.0 1.0 0.0 0 0 0 0)
      (Class|RadialForceComponent|FireImpulse (Variables|Default|GetRadialForce))
      (Actor|DestroyActor))))

(event EventBeginPlay)

(event Game|Damage|EventRadialDamage
  (params (DamageReceived :type Float%20%28single-precision%29) (DamageType :type Damage%20Type%20Object%20Reference) (Origin :type Vector :default "0, 0, 0") (HitInfo :type Hit%20Result%20Structure%20%28by%20ref%29) (InstigatedBy :type Controller%20Object%20Reference) (DamageCauser :type Actor%20Object%20Reference))
  (Actor|DestroyActor)
  (Effects|SpawnEmitteratLocation "/Game/StarterContent/Particles/P_Explosion.P_Explosion" (Transformation|GetActorLocation) "0, 0, 0" "3.000000,3.000000,3.000000"))

(event Game|Damage|EventAnyDamage
  (params (Damage :type Float%20%28single-precision%29) (DamageType :type Damage%20Type%20Object%20Reference) (InstigatedBy :type Controller%20Object%20Reference) (DamageCauser :type Actor%20Object%20Reference))
  (bind _output_get (Variables|Default|SetTripwireHealth (- (Variables|Default|GetTripwireHealth) Damage)))
  (if (<= _output_get 0.0)
    (for _index (range 0 (Math|Random|RandomInteger 2))
      (Game|Damage|ApplyRadialDamage 1e+02 (Transformation|GetActorLocation) 5e+02 0 0 self 0 false "ECC_Visibility")
      (Default|PlayerGotDamage (Variables|Default|GetPlayer))
      (Effects|SpawnEmitteratLocation "/Game/StarterContent/Particles/P_Explosion.P_Explosion" (Transformation|GetActorLocation) "0, 0, 0" "3.000000,3.000000,3.000000")
      (Audio|PlaySoundatLocation "/Game/Sound/SoundEffect/Audio/Explosion_Cue.Explosion_Cue" (Transformation|GetActorLocation) "0, 0, 0" 1.0 1.0 0.0 0 0 0 0)
      (Class|RadialForceComponent|FireImpulse (Variables|Default|GetRadialForce)))
    (Actor|DestroyActor)))

(fn ConstructionScript)